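; Game mode for a two-player 3D chess game that assigns player indices and starts the first turn through the chess game state.
; BeginPlay always runs local setup for player zero, while PostLogin waits briefly after two players join, then indexes both and begins the networked turn.
; It also exposes local-mode accessors and runs a Delay-throttled Tick clock whose seconds and minutes never reset.
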(event `self.K2_PostLogin`
  (params (NewPlayer :type "PlayerController Object Reference"))
  (`parent.K2_PostLogin` NewPlayer)
  (bind _returnvalue (`self.GetNumPlayers`))
  (if (== _returnvalue 2)
    (`KismetSystemLibrary.Delay` 2.0)
    (`|ExecutionSequence`
      (:`then_0`
        (`self.Create Player`)
        (set `self.PlayerAmt` 2))
      (:`then_1`
        (`/Game/3DGame/Millinium3DChess/BluePrints/MChessGameState.BeginPlayerTurn` (cast `/Game/3DGame/Millinium3DChess/BluePrints/MChessGameState` (`GameplayStatics.GetGameState`) :!pure true) 0)))))

(event `self.ReceiveTick`
  (params (DeltaSeconds :type "Float (single-precision)"))
  (`KismetSystemLibrary.Delay` 1.0)
  (set `self.Seconds` (+ (`self.Seconds`) 1))
  (if (> (`self.Seconds`) 59)
    (set `self.Minutes` (+ (`self.Minutes`) 1))
    (if (> (`self.Minutes`) 23)
      (set `self.Hours` (+ (`self.Hours`) 1)))))

(event `self.ReceiveBeginPlay`
  (if true
    (if (== 2 2)
      (`|ExecutionSequence`
        (:`then_0`
          (`KismetSystemLibrary.PrintString` "Creating The Player")
          (`/Game/3DGame/Millinium3DChess/BluePrints/MPlayerController.SetPlayerIndex (Local)` (cast `/Game/3DGame/Millinium3DChess/BluePrints/MPlayerController` (`GameplayStatics.GetPlayerController` 0) :!pure true) 0))
        (:`then_1`
          (`/Game/3DGame/Millinium3DChess/BluePrints/MChessGameState.BeginPlayerTurn(Local)` (cast `/Game/3DGame/Millinium3DChess/BluePrints/MChessGameState` (`GameplayStatics.GetGameState`) :!pure true) 0)
          (`KismetSystemLibrary.PrintString` "Turn Started"))))))

(fn `Create Player`
  (`/Game/3DGame/Millinium3DChess/BluePrints/MPlayerController.SetPlayerIndex (client)` (cast `/Game/3DGame/Millinium3DChess/BluePrints/MPlayerController` (`GameplayStatics.GetPlayerController` 0) :!pure true) 0)
  (`/Game/3DGame/Millinium3DChess/BluePrints/MPlayerController.SetPlayerIndex (client)` (cast `/Game/3DGame/Millinium3DChess/BluePrints/MPlayerController` (`GameplayStatics.GetPlayerController` 1) :!pure true) 1))

(fn `GetLocalMode`
  (returns (LocalMode :type Boolean) (PlayerAmount :type Integer))
  (return (`self.IsLocalGame`) (`self.PlayerAmt`)))

(fn `SetLocalMode`
  (params (IsLocalGame :type Boolean))
  (set `self.IsLocalGame` IsLocalGame)
  (set `self.PlayerAmt` 2)
  (`KismetSystemLibrary.PrintString` "Local Mode and player amt are set"))

(fn `UserConstructionScript`)