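; Game mode for four-player chess that assigns player indices and starts the first turn through the game state.
; When a fourth player logs in, it waits briefly, indexes all four controllers and begins turn 0.
; BeginPlay always runs the local-game start for controller 0, as its checks are hard-coded rather than reading the local-mode flag.
; Tick drives a delay-based time counter whose values never reset.
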(event `self.K2_PostLogin`
  (params (NewPlayer :type "PlayerController Object Reference"))
  (`parent.K2_PostLogin` NewPlayer)
  (bind _returnvalue (`self.GetNumPlayers`))
  (if (== _returnvalue 4)
    (`KismetSystemLibrary.Delay` 3.0)
    (`|ExecutionSequence`
      (:`then_0`
        (`self.CreatePlayer`))
      (:`then_1`
        (`/Game/4PGame/BluePrints/4PChessGameState.BeginPlayerTurn` (cast `/Game/4PGame/BluePrints/4PChessGameState` (`GameplayStatics.GetGameState`) :!pure true) 0)))))

(event `self.ReceiveTick`
  (params (DeltaSeconds :type "Float (single-precision)"))
  (`KismetSystemLibrary.Delay` 1.0)
  (set `self.Seconds` (+ (`self.Seconds`) 1))
  (if (> (`self.Seconds`) 59)
    (set `self.Minutes` (+ (`self.Minutes`) 1))
    (if (> (`self.Minutes`) 23)
      (set `self.Hours` (+ (`self.Hours`) 1)))))

(event `self.ReceiveBeginPlay`
  (if true
    (if (== 4 4)
      (`|ExecutionSequence`
        (:`then_0`
          (`KismetSystemLibrary.PrintString` "Creating The Player")
          (`/Game/4PGame/BluePrints/4PPlayerController.SetPlayerIndex(Local)` (cast `/Game/4PGame/BluePrints/4PPlayerController` (`GameplayStatics.GetPlayerController` 0) :!pure true) 0))
        (:`then_1`
          (`/Game/4PGame/BluePrints/4PChessGameState.BeginPlayerTurn(Local)` (cast `/Game/4PGame/BluePrints/4PChessGameState` (`GameplayStatics.GetGameState`) :!pure true) 0)
          (`KismetSystemLibrary.PrintString` "Turn Started"))))))

(fn `CreatePlayer`
  (`/Game/4PGame/BluePrints/4PPlayerController.SetPlayerIndex (client)` (cast `/Game/4PGame/BluePrints/4PPlayerController` (`GameplayStatics.GetPlayerController` 0) :!pure true) 0)
  (`/Game/4PGame/BluePrints/4PPlayerController.SetPlayerIndex (client)` (cast `/Game/4PGame/BluePrints/4PPlayerController` (`GameplayStatics.GetPlayerController` 1) :!pure true) 1)
  (`/Game/4PGame/BluePrints/4PPlayerController.SetPlayerIndex (client)` (cast `/Game/4PGame/BluePrints/4PPlayerController` (`GameplayStatics.GetPlayerController` 2) :!pure true) 2)
  (`/Game/4PGame/BluePrints/4PPlayerController.SetPlayerIndex (client)` (cast `/Game/4PGame/BluePrints/4PPlayerController` (`GameplayStatics.GetPlayerController` 3) :!pure true) 3))

(fn `GetLocalMode`
  (returns (LocalMode :type Boolean) (PlayerAmount :type Integer))
  (return (`self.IsLocalGame`) (`self.PlayerAmt`)))

(fn `SetLocalMode`
  (params (IsLocalGame :type Boolean))
  (set `self.IsLocalGame` IsLocalGame)
  (set `self.PlayerAmt` 4)
  (`KismetSystemLibrary.PrintString` "Local Mode and player amt are set"))

(fn `UserConstructionScript`)