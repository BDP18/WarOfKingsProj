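; MChessLibrary is a Blueprint function library of shared helpers for the Millinium 3D chess game.
; PlayerColor maps a player index to white or near-black, and OpponentColor reuses it with the index flipped.
; The remaining helpers cast the game state to reach the board, or the game mode to read local mode and player amount.
; SetLocalMode takes no value and always passes false to the game mode.
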(fn `Board`
  (returns (Board :type "/Game/3DGame/Millinium3DChess/BluePrints/Board/MBoard Object Reference"))
  (return (`/Game/3DGame/Millinium3DChess/BluePrints/MChessGameState.GetBoard` (`self.ChessGameState` (`local.__WorldContext`)))))

(fn `ChessGameState`
  (returns (`Chess Game State` :type "/Game/3DGame/Millinium3DChess/BluePrints/MChessGameState Object Reference"))
  (return (cast `/Game/3DGame/Millinium3DChess/BluePrints/MChessGameState` (`GameplayStatics.GetGameState` (`local.__WorldContext`)) :!pure true)))

(fn `GetLocalMode`
  (returns (`Local Mode` :type Boolean) (PlayerAmount :type Integer))
  (bind (_localmode _playeramount) (`/Game/3DGame/Millinium3DChess/BluePrints/MChessGameMode.GetLocalMode` (cast `/Game/3DGame/Millinium3DChess/BluePrints/MChessGameMode` (`GameplayStatics.GetGameMode` (`local.__WorldContext`)) :!pure true)))
  (return _localmode _playeramount))

(fn `OpponentColor`
  (params (PlayerIndex :type Integer))
  (returns (Color :type "LinearColor Structure"))
  (return (`self.PlayerColor` (select `int` PlayerIndex :`0` 1 :`1` 0) (`local.__WorldContext`))))

(fn `PlayerColor`
  (params (PlayerIndex :type Integer))
  (returns (Color :type "LinearColor Structure") (__WorldContext1 :type "Object Object Reference"))
  (return (select `int` PlayerIndex :`0` (struct :`R` 1.0 :`G` 1.0 :`B` 1.0 :`A` 1.0) :`1` (struct :`R` 0.01 :`G` 0.01 :`B` 0.01 :`A` 1.0) :!type "LinearColor Structure") (`local.__WorldContext`)))

(fn `SetLocalMode`
  (`KismetSystemLibrary.PrintString` null "Set Local Mode in library")
  (`/Game/3DGame/Millinium3DChess/BluePrints/MChessGameMode.SetLocalMode` (cast `/Game/3DGame/Millinium3DChess/BluePrints/MChessGameMode` (`GameplayStatics.GetGameMode` (`local.__WorldContext`)) :!pure true) false))