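; Game mode for three-player chess that assigns player indices and starts the first turn through 3PChessGameState.
; Once three players log in, it waits briefly, sets all three controllers to index 0 via CreatePlayer, then begins the networked turn.
; BeginPlay also always starts a local turn for the first controller, without checking the local-mode flag.
; Tick uses a Delay to count seconds, feeding minute and hour counters that never reset.
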(event `self.K2_PostLogin`
  (params (NewPlayer :type "PlayerController Object Reference"))
  (`parent.K2_PostLogin` NewPlayer)
  (bind _returnvalue (`self.GetNumPlayers`))
  (if (== _returnvalue 3)
    (`KismetSystemLibrary.Delay` 3.0)
    (`|ExecutionSequence`
      (:`then_0`
        (`self.CreatePlayer`))
      (:`then_1`
        (`/Game/3PGame/Blueprints/3PChessGameState.BeginPlayerTurn` (cast `/Game/3PGame/Blueprints/3PChessGameState` (`GameplayStatics.GetGameState`) :!pure true) 0)))))

(event `self.ReceiveTick`
  (params (DeltaSeconds :type "Float (single-precision)"))
  (`KismetSystemLibrary.Delay` 1.0)
  (set `self.Seconds` (+ (`self.Seconds`) 1))
  (if (> (`self.Seconds`) 59)
    (set `self.Minutes` (+ (`self.Minutes`) 1))
    (if (> (`self.Minutes`) 23)
      (set `self.Hours` (+ (`self.Hours`) 1)))))

(event `self.ReceiveBeginPlay`
  (if true
    (if (== 3 3)
      (`|ExecutionSequence`
        (:`then_0`
          (`KismetSystemLibrary.PrintString` "Creating The Player")
          (`/Game/3PGame/Blueprints/3PPlayerController.SetPlayerIndex (Local)` (cast `/Game/3PGame/Blueprints/3PPlayerController` (`GameplayStatics.GetPlayerController` 0) :!pure true) 0))
        (:`then_1`
          (`/Game/3PGame/Blueprints/3PChessGameState.BeginPlayerTurn(Local)` (cast `/Game/3PGame/Blueprints/3PChessGameState` (`GameplayStatics.GetGameState`) :!pure true) 0)
          (`KismetSystemLibrary.PrintString` "Turn Started"))))))

(fn `CreatePlayer`
  (`/Game/3PGame/Blueprints/3PPlayerController.SetPlayerIndex (client)` (cast `/Game/3PGame/Blueprints/3PPlayerController` (`GameplayStatics.GetPlayerController` 0) :!pure true) 0)
  (`/Game/3PGame/Blueprints/3PPlayerController.SetPlayerIndex (client)` (cast `/Game/3PGame/Blueprints/3PPlayerController` (`GameplayStatics.GetPlayerController` 1) :!pure true) 0)
  (`/Game/3PGame/Blueprints/3PPlayerController.SetPlayerIndex (client)` (cast `/Game/3PGame/Blueprints/3PPlayerController` (`GameplayStatics.GetPlayerController` 2) :!pure true) 0))

(fn `GetLocalMode`
  (returns (LocalMode :type Boolean) (PlayerAmount :type Integer))
  (return (`self.IsLocalGame`) (`self.PlayerAmt`)))

(fn `SetLocalMode`
  (set `self.IsLocalGame` true)
  (set `self.PlayerAmt` 3)
  (`KismetSystemLibrary.PrintString` "Local Mode and player amt are set"))

(fn `UserConstructionScript`)