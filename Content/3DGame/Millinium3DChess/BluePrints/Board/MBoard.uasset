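; Board actor for a three-level 3D chess game that spawns both sides' pieces at BeginPlay, player 0 on the top level and player 1 on the bottom.
; A flat BoardState array stores pieces by cell, with helpers converting between cells and world positions.
; IsMoveAvailable checks the piece's potential move list, while MakeMove teleports the piece, destroys any occupant and updates the array.
; The BeginPlay authority check is bypassed by a constant-true branch.
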(event `self.ReceiveBeginPlay`
  (if (not true)
    (`/Engine/EditorBlueprintResources/ActorMacros.Switch Has Authority` ; Must Stay Here. Handles replication between client and server
      (:`Authority`
        _)))
  (`KismetArrayLibrary.Array_Resize` (`self.BoardState`) 192)
  (for _index (range 2)
    (`self.MakeKings` _index)
    (`self.MakeQueens` _index)
    (`self.MakeBishops` _index)
    (`self.MakeKnights` _index)
    (`self.MakeRooks` _index)
    (`self.MakePawns` _index)))

(fn `AddPiece`
  (params (Piece :type "/Game/3DGame/Millinium3DChess/BluePrints/Pieces/MPiece Object Reference") (Cell :type "/Game/3DGame/Millinium3DChess/BluePrints/Board/MCell Structure"))
  (`KismetArrayLibrary.Array_Set` (`self.BoardState`) (`self.GetIndexFromCell` Cell) Piece))

(fn `BoardStateElem`
  (params (`Dimension 1` :type Integer))
  (returns (Output :type "/Game/3DGame/Millinium3DChess/BluePrints/Pieces/MPiece Object Reference"))
  (return (`|GetArrayItem` (`self.BoardState`) `Dimension 1`)))

(fn `CellToGrid`
  (params (Cell :type "/Game/3DGame/Millinium3DChess/BluePrints/Board/MCell Structure"))
  (returns (ReturnValue :type "Vector Structure"))
  (return (+ (`KismetMathLibrary.MakeVector` (`self.HandleRow` Cell_Y_8_A31AD37F4ABEE7282C2022A30B0EBA3F) (`self.HandleColumn` Cell_X_7_767D76F24B6395F8CD2202A2E588D57E) (`self.HandleHeight` Cell_Z_9_A0ABD97541C337FF31685EB1A05A7A38)) (`self.GridVector`))))

(fn `GetBoardState`
  (returns (BoardState :type "Array of /Game/3DGame/Millinium3DChess/BluePrints/Pieces/MPiece Object Reference"))
  (return (`self.BoardState`)))

(fn `GetBoardStateSize`
  (returns (ReturnValue :type Integer))
  (return (`KismetArrayLibrary.Array_Length` (`self.BoardState`))))

(fn `GetCellInfo`
  (params (Cell :type "/Game/3DGame/Millinium3DChess/BluePrints/Board/MCell Structure"))
  (returns (TileValid :type Boolean) (TileFree :type Boolean) (BoardPiece :type "/Game/3DGame/Millinium3DChess/BluePrints/Pieces/MPiece Object Reference"))
  (bind _piece (`self.PieceAtLocation` (`local.Cell`)))
  (if (`self.IsCellInRange` Cell)
    (return true (not (`KismetSystemLibrary.IsValid` _piece)) _piece)
    (else
      (return false false null))))

(fn `IsCellInRange`
  (params (Cell :type "/Game/3DGame/Millinium3DChess/BluePrints/Board/MCell Structure"))
  (returns (InRange :type Boolean))
  (return (and (and (`KismetMathLibrary.InRange_IntInt` Cell_X_7_767D76F24B6395F8CD2202A2E588D57E 0 7) (`KismetMathLibrary.InRange_IntInt` Cell_Y_8_A31AD37F4ABEE7282C2022A30B0EBA3F 0 7)) (`KismetMathLibrary.InRange_IntInt` Cell_Z_9_A0ABD97541C337FF31685EB1A05A7A38 0 2))))

(fn `IsMoveAvailable`
  (params (StartCell :type "/Game/3DGame/Millinium3DChess/BluePrints/Board/MCell Structure") (EndCell :type "/Game/3DGame/Millinium3DChess/BluePrints/Board/MCell Structure"))
  (returns (Result :type Boolean))
  (locals (SelectedPiece :type "/Game/3DGame/Millinium3DChess/BluePrints/Pieces/MPiece Object Reference"))
  (bind _output_get (set `local.SelectedPiece` (`self.PieceAtLocation` StartCell)))
  (`/Engine/EditorBlueprintResources/StandardMacros.IsValid` _output_get
    (:`Is Valid`
      (return (`KismetArrayLibrary.Array_Contains` (`/Game/3DGame/Millinium3DChess/BluePrints/Pieces/MPiece.PotentialMoveList` (`local.SelectedPiece`) (`local.StartCell`)) (`local.EndCell`))))
    (:`Is Not Valid`
      (return false))))

(fn `MakeBishops`
  (params (`Player Index` :type Integer))
  (locals (Col :type Integer) (Row :type Integer))
  (bind _player_index (`local.Player Index`))
  (bind _player_index_2 (`local.Player Index`))
  (bind _returnvalue (== _player_index 0))
  (bind _returnvalue_2 (== _player_index_2 1))
  (set `local.Row` (select `int` (`local.Player Index`) :`0` 0 :`1` 7))
  (`|ExecutionSequence`
    (:`then_0`
      (if _returnvalue_2
        (set `local.Col` (select `int` _player_index_2 :`0` 2 :`1` 5))
        (bind _returnvalue_3 (`|SpawnActorFromClass` "/Game/3DGame/Millinium3DChess/BluePrints/Pieces/MBishop.MBishop_C" (`KismetMathLibrary.MakeTransform` (`self.CellToGrid` (make `/Game/3DGame/Millinium3DChess/BluePrints/Board/MCell` (`local.Col`) (`local.Row`)))) "Undefined" "OverrideRootScale" null (`local.Player Index`) null))
        (`self.AddPiece` _returnvalue_3 (make `/Game/3DGame/Millinium3DChess/BluePrints/Board/MCell` (`local.Col`) (`local.Row`)))))
    (:`then_1`
      (if _returnvalue_2
        (set `local.Col` (select `int` (`local.Player Index`) :`0` 5 :`1` 2))
        (bind _returnvalue_4 (`|SpawnActorFromClass` "/Game/3DGame/Millinium3DChess/BluePrints/Pieces/MBishop.MBishop_C" (`KismetMathLibrary.MakeTransform` (`self.CellToGrid` (make `/Game/3DGame/Millinium3DChess/BluePrints/Board/MCell` (`local.Col`) (`local.Row`)))) "Undefined" "OverrideRootScale" null (`local.Player Index`) null))
        (`self.AddPiece` _returnvalue_4 (make `/Game/3DGame/Millinium3DChess/BluePrints/Board/MCell` (`local.Col`) (`local.Row`)))))
    (:`then_2`
      (if _returnvalue
        (set `local.Col` (select `int` _player_index :`0` 2 :`1` 5))
        (bind _returnvalue_5 (`|SpawnActorFromClass` "/Game/3DGame/Millinium3DChess/BluePrints/Pieces/MBishop.MBishop_C" (`KismetMathLibrary.MakeTransform` (`self.CellToGrid` (make `/Game/3DGame/Millinium3DChess/BluePrints/Board/MCell` (`local.Col`) (`local.Row`) 2))) "Undefined" "OverrideRootScale" null (`local.Player Index`) null))
        (`self.AddPiece` _returnvalue_5 (make `/Game/3DGame/Millinium3DChess/BluePrints/Board/MCell` (`local.Col`) (`local.Row`) 2))))
    (:`then_3`
      (if _returnvalue
        (set `local.Col` (select `int` (`local.Player Index`) :`0` 5 :`1` 2))
        (bind _returnvalue_6 (`|SpawnActorFromClass` "/Game/3DGame/Millinium3DChess/BluePrints/Pieces/MBishop.MBishop_C" (`KismetMathLibrary.MakeTransform` (`self.CellToGrid` (make `/Game/3DGame/Millinium3DChess/BluePrints/Board/MCell` (`local.Col`) (`local.Row`) 2))) "Undefined" "OverrideRootScale" null (`local.Player Index`) null))
        (`self.AddPiece` _returnvalue_6 (make `/Game/3DGame/Millinium3DChess/BluePrints/Board/MCell` (`local.Col`) (`local.Row`) 2))))))

(fn `MakeKings`
  (params (`Player Index` :type Integer))
  (locals (Col :type Integer) (Row :type Integer))
  (bind _player_index (`local.Player Index`))
  (bind _player_index_2 (`local.Player Index`))
  (`|ExecutionSequence`
    (:`then_0`
      (if (== _player_index_2 1)
        (set `local.Row` (select `int` _player_index_2 :`0` 0 :`1` 7))
        (set `local.Col` 4)
        (bind _returnvalue (`|SpawnActorFromClass` "/Game/3DGame/Millinium3DChess/BluePrints/Pieces/MKing.MKing_C" (`KismetMathLibrary.MakeTransform` (`self.CellToGrid` (make `/Game/3DGame/Millinium3DChess/BluePrints/Board/MCell` (`local.Col`) (`local.Row`)))) "Undefined" "OverrideRootScale" null (`local.Player Index`) null))
        (`self.AddPiece` _returnvalue (make `/Game/3DGame/Millinium3DChess/BluePrints/Board/MCell` (`local.Col`) (`local.Row`)))))
    (:`then_1`
      (if (== _player_index 0)
        (set `local.Row` (select `int` _player_index :`0` 0 :`1` 7))
        (set `local.Col` 4)
        (bind _returnvalue_2 (`|SpawnActorFromClass` "/Game/3DGame/Millinium3DChess/BluePrints/Pieces/MKing.MKing_C" (`KismetMathLibrary.MakeTransform` (`self.CellToGrid` (make `/Game/3DGame/Millinium3DChess/BluePrints/Board/MCell` (`local.Col`) (`local.Row`) 2))) "Undefined" "OverrideRootScale" null (`local.Player Index`) null))
        (`self.AddPiece` _returnvalue_2 (make `/Game/3DGame/Millinium3DChess/BluePrints/Board/MCell` (`local.Col`) (`local.Row`) 2))))))

(fn `MakeKnights`
  (params (PlayerIndex :type Integer))
  (locals (Col :type Integer) (Row :type Integer))
  (bind _playerindex (`local.PlayerIndex`))
  (bind _playerindex_2 (`local.PlayerIndex`))
  (bind _returnvalue (== _playerindex 0))
  (bind _returnvalue_2 (== _playerindex_2 1))
  (set `local.Row` (select `int` (`local.PlayerIndex`) :`0` 0 :`1` 7))
  (`|ExecutionSequence`
    (:`then_0`
      (if _returnvalue_2
        (set `local.Col` (select `int` _playerindex_2 :`0` 1 :`1` 6))
        (bind _returnvalue_3 (`|SpawnActorFromClass` "/Game/3DGame/Millinium3DChess/BluePrints/Pieces/MKnight.MKnight_C" (`KismetMathLibrary.MakeTransform` (`self.CellToGrid` (make `/Game/3DGame/Millinium3DChess/BluePrints/Board/MCell` (`local.Col`) (`local.Row`)))) "Undefined" "OverrideRootScale" null (`local.PlayerIndex`) null))
        (`self.AddPiece` _returnvalue_3 (make `/Game/3DGame/Millinium3DChess/BluePrints/Board/MCell` (`local.Col`) (`local.Row`)))))
    (:`then_1`
      (if _returnvalue_2
        (set `local.Col` (select `int` (`local.PlayerIndex`) :`0` 6 :`1` 1))
        (bind _returnvalue_4 (`|SpawnActorFromClass` "/Game/3DGame/Millinium3DChess/BluePrints/Pieces/MKnight.MKnight_C" (`KismetMathLibrary.MakeTransform` (`self.CellToGrid` (make `/Game/3DGame/Millinium3DChess/BluePrints/Board/MCell` (`local.Col`) (`local.Row`)))) "Undefined" "OverrideRootScale" null (`local.PlayerIndex`) null))
        (`self.AddPiece` _returnvalue_4 (make `/Game/3DGame/Millinium3DChess/BluePrints/Board/MCell` (`local.Col`) (`local.Row`)))))
    (:`then_2`
      (if _returnvalue
        (set `local.Col` (select `int` _playerindex :`0` 1 :`1` 6))
        (bind _returnvalue_5 (`|SpawnActorFromClass` "/Game/3DGame/Millinium3DChess/BluePrints/Pieces/MKnight.MKnight_C" (`KismetMathLibrary.MakeTransform` (`self.CellToGrid` (make `/Game/3DGame/Millinium3DChess/BluePrints/Board/MCell` (`local.Col`) (`local.Row`) 2))) "Undefined" "OverrideRootScale" null (`local.PlayerIndex`) null))
        (`self.AddPiece` _returnvalue_5 (make `/Game/3DGame/Millinium3DChess/BluePrints/Board/MCell` (`local.Col`) (`local.Row`) 2))))
    (:`then_3`
      (if _returnvalue
        (set `local.Col` (select `int` (`local.PlayerIndex`) :`0` 6 :`1` 1))
        (bind _returnvalue_6 (`|SpawnActorFromClass` "/Game/3DGame/Millinium3DChess/BluePrints/Pieces/MKnight.MKnight_C" (`KismetMathLibrary.MakeTransform` (`self.CellToGrid` (make `/Game/3DGame/Millinium3DChess/BluePrints/Board/MCell` (`local.Col`) (`local.Row`) 2))) "Undefined" "OverrideRootScale" null (`local.PlayerIndex`) null))
        (`self.AddPiece` _returnvalue_6 (make `/Game/3DGame/Millinium3DChess/BluePrints/Board/MCell` (`local.Col`) (`local.Row`) 2))))))

(fn `MakeMove`
  (params (StartCell :type "/Game/3DGame/Millinium3DChess/BluePrints/Board/MCell Structure") (EndCell :type "/Game/3DGame/Millinium3DChess/BluePrints/Board/MCell Structure"))
  (locals (SelectedPiece :type "/Game/3DGame/Millinium3DChess/BluePrints/Pieces/MPiece Object Reference") (EndPiece :type "/Game/3DGame/Millinium3DChess/BluePrints/Pieces/MPiece Object Reference"))
  (set `local.SelectedPiece` (`self.PieceAtLocation` StartCell))
  (set `local.EndPiece` (`self.PieceAtLocation` EndCell))
  (`self.K2_SetActorLocation` (`local.SelectedPiece`) (`self.CellToGrid` (`local.EndCell`)) false true)
  (bind _endpiece (`local.EndPiece`)
    (:`then`
      (`self.K2_DestroyActor` _endpiece))
    (:`else`
      _))
  (`self.MovePiece` (`local.StartCell`) (`local.EndCell`)))

(fn `MakePawns`
  (params (PlayerIndex :type Integer))
  (locals (Row :type Integer) (Col :type Integer))
  (if (== (`local.PlayerIndex`) 0)
    (set `local.Row` (select `int` (`local.PlayerIndex`) :`0` 1 :`1` 6))
    (for _index (range 8)
      (bind _output_get (set `local.Col` _index))
      (bind _returnvalue (`|SpawnActorFromClass` "/Game/3DGame/Millinium3DChess/BluePrints/Pieces/MPawn.MPawn_C" (`KismetMathLibrary.MakeTransform` (`self.CellToGrid` (make `/Game/3DGame/Millinium3DChess/BluePrints/Board/MCell` _output_get (`local.Row`) 2))) "Undefined" "OverrideRootScale" null (`local.PlayerIndex`) null))
      (`self.AddPiece` _returnvalue (make `/Game/3DGame/Millinium3DChess/BluePrints/Board/MCell` (`local.Col`) (`local.Row`) 2)))
    (else
      (set `local.Row` (select `int` (`local.PlayerIndex`) :`0` 1 :`1` 6))
      (for _index_2 (range 8)
        (bind _output_get_2 (set `local.Col` _index_2))
        (bind _returnvalue_2 (`|SpawnActorFromClass` "/Game/3DGame/Millinium3DChess/BluePrints/Pieces/MPawn.MPawn_C" (`KismetMathLibrary.MakeTransform` (`self.CellToGrid` (make `/Game/3DGame/Millinium3DChess/BluePrints/Board/MCell` _output_get_2 (`local.Row`)))) "Undefined" "OverrideRootScale" null (`local.PlayerIndex`) null))
        (`self.AddPiece` _returnvalue_2 (make `/Game/3DGame/Millinium3DChess/BluePrints/Board/MCell` (`local.Col`) (`local.Row`)))))))

(fn `MakeQueens`
  (params (`Player Index` :type Integer))
  (locals (Col :type Integer) (Row :type Integer))
  (bind _player_index (`local.Player Index`))
  (`|ExecutionSequence`
    (:`then_0`
      (if (== _player_index 1)
        (set `local.Row` (select `int` _player_index :`0` 0 :`1` 7))
        (set `local.Col` 3)
        (bind _returnvalue (`|SpawnActorFromClass` "/Game/3DGame/Millinium3DChess/BluePrints/Pieces/MQueen.MQueen_C" (`KismetMathLibrary.MakeTransform` (`self.CellToGrid` (make `/Game/3DGame/Millinium3DChess/BluePrints/Board/MCell` (`local.Col`) (`local.Row`)))) "Undefined" "OverrideRootScale" null (`local.Player Index`) null))
        (`self.AddPiece` _returnvalue (make `/Game/3DGame/Millinium3DChess/BluePrints/Board/MCell` (`local.Col`) (`local.Row`)))))
    (:`then_1`
      (if (== _player_index 0)
        (set `local.Row` (select `int` (`local.Player Index`) :`0` 0 :`1` 7))
        (set `local.Col` 3)
        (bind _returnvalue_2 (`|SpawnActorFromClass` "/Game/3DGame/Millinium3DChess/BluePrints/Pieces/MQueen.MQueen_C" (`KismetMathLibrary.MakeTransform` (`self.CellToGrid` (make `/Game/3DGame/Millinium3DChess/BluePrints/Board/MCell` (`local.Col`) (`local.Row`) 2))) "Undefined" "OverrideRootScale" null (`local.Player Index`) null))
        (`self.AddPiece` _returnvalue_2 (make `/Game/3DGame/Millinium3DChess/BluePrints/Board/MCell` (`local.Col`) (`local.Row`) 2))))))

(fn `MakeRooks`
  (params (`Player Index` :type Integer))
  (locals (Col :type Integer) (Row :type Integer))
  (bind _player_index (`local.Player Index`))
  (bind _returnvalue (== (`local.Player Index`) 1))
  (bind _returnvalue_2 (== _player_index 0))
  (set `local.Row` (select `int` (`local.Player Index`) :`0` 0 :`1` 7))
  (`|ExecutionSequence`
    (:`then_0`
      (if _returnvalue_2
        (set `local.Col` (select `int` _player_index :`0` 2 :`1` 0))
        (bind _returnvalue_3 (`|SpawnActorFromClass` "/Game/3DGame/Millinium3DChess/BluePrints/Pieces/MRook.MRook_C" (`KismetMathLibrary.MakeTransform` (`self.CellToGrid` (make `/Game/3DGame/Millinium3DChess/BluePrints/Board/MCell` 0 (`local.Row`) (`local.Col`)))) "Undefined" "OverrideRootScale" null (`local.Player Index`) null))
        (`self.AddPiece` _returnvalue_3 (make `/Game/3DGame/Millinium3DChess/BluePrints/Board/MCell` 0 (`local.Row`) (`local.Col`)))))
    (:`then_1`
      (if _returnvalue_2
        (set `local.Col` (select `int` (`local.Player Index`) :`0` 2 :`1` 0))
        (bind _returnvalue_4 (`|SpawnActorFromClass` "/Game/3DGame/Millinium3DChess/BluePrints/Pieces/MRook.MRook_C" (`KismetMathLibrary.MakeTransform` (`self.CellToGrid` (make `/Game/3DGame/Millinium3DChess/BluePrints/Board/MCell` 7 (`local.Row`) (`local.Col`)))) "Undefined" "OverrideRootScale" null (`local.Player Index`) null))
        (`self.AddPiece` _returnvalue_4 (make `/Game/3DGame/Millinium3DChess/BluePrints/Board/MCell` 7 (`local.Row`) (`local.Col`)))))
    (:`then_2`
      (if _returnvalue
        (set `local.Col` (select `int` (`local.Player Index`) :`0` 0 :`1` 7))
        (bind _returnvalue_5 (`|SpawnActorFromClass` "/Game/3DGame/Millinium3DChess/BluePrints/Pieces/MRook.MRook_C" (`KismetMathLibrary.MakeTransform` (`self.CellToGrid` (make `/Game/3DGame/Millinium3DChess/BluePrints/Board/MCell` (`local.Col`) (`local.Row`)))) "Undefined" "OverrideRootScale" null (`local.Player Index`) null))
        (`self.AddPiece` _returnvalue_5 (make `/Game/3DGame/Millinium3DChess/BluePrints/Board/MCell` (`local.Col`) (`local.Row`)))))
    (:`then_3`
      (if _returnvalue
        (set `local.Col` (select `int` (`local.Player Index`) :`0` 7 :`1` 0))
        (bind _returnvalue_6 (`|SpawnActorFromClass` "/Game/3DGame/Millinium3DChess/BluePrints/Pieces/MRook.MRook_C" (`KismetMathLibrary.MakeTransform` (`self.CellToGrid` (make `/Game/3DGame/Millinium3DChess/BluePrints/Board/MCell` (`local.Col`) (`local.Row`)))) "Undefined" "OverrideRootScale" null (`local.Player Index`) null))
        (`self.AddPiece` _returnvalue_6 (make `/Game/3DGame/Millinium3DChess/BluePrints/Board/MCell` (`local.Col`) (`local.Row`)))))))

(fn `MovePiece`
  (params (StartCells :type "/Game/3DGame/Millinium3DChess/BluePrints/Board/MCell Structure") (EndCells :type "/Game/3DGame/Millinium3DChess/BluePrints/Board/MCell Structure"))
  (locals (PieceToMove :type "/Game/3DGame/Millinium3DChess/BluePrints/Pieces/MPiece Object Reference"))
  (set `local.PieceToMove` (`self.PieceAtLocation` StartCells))
  (`KismetArrayLibrary.Array_Set` (`self.BoardState`) (`self.GetIndexFromCell` (`local.StartCells`)))
  (`KismetArrayLibrary.Array_Set` (`self.BoardState`) (`self.GetIndexFromCell` (`local.EndCells`)) (`local.PieceToMove`))
  (`/Game/3DGame/Millinium3DChess/BluePrints/Pieces/MPiece.WhenMoved` (`local.PieceToMove`)))

(fn `PieceAtLocation`
  (params (Cell :type "/Game/3DGame/Millinium3DChess/BluePrints/Board/MCell Structure"))
  (returns (Piece :type "/Game/3DGame/Millinium3DChess/BluePrints/Pieces/MPiece Object Reference"))
  (bind _output (`|GetArrayItem` (`self.BoardState`) (`self.GetIndexFromCell` Cell)))
  (`KismetSystemLibrary.PrintString` (`KismetSystemLibrary.GetDisplayName` _output))
  (return _output))

(fn `UserConstructionScript`)

(fn `WorldToGrid`
  (params (WorldLocation :type "Vector Structure"))
  (returns (Cell :type "/Game/3DGame/Millinium3DChess/BluePrints/Board/MCell Structure") (InBounds :type Boolean))
  (locals (`Column Cell` :type Integer) (`Row Cell` :type Integer) (HeightCell :type Integer))
  (bind _lengthofcell (`self.LengthOfCell`))
  (bind (_returnvalue_x _returnvalue_y _returnvalue_z) (`KismetMathLibrary.BreakVector` (- (`local.WorldLocation`) (`self.GridVector`))))
  (`|ExecutionSequence`
    (:`then_0`
      (if true
        (set `local.Column Cell` (`KismetMathLibrary.FFloor` (/ _returnvalue_y _lengthofcell)))
        (set `local.Row Cell` (`KismetMathLibrary.FFloor` (/ _returnvalue_x _lengthofcell)))
        (set `local.HeightCell` (`KismetMathLibrary.FFloor` (/ _returnvalue_z 800.0)))))
    (:`then_1`
      (if (`self.IsCellInRange` (make `/Game/3DGame/Millinium3DChess/BluePrints/Board/MCell` (`local.Column Cell`) (`local.Row Cell`) (`local.HeightCell`)))
        (return (make `/Game/3DGame/Millinium3DChess/BluePrints/Board/MCell` (`local.Column Cell`) (`local.Row Cell`) (`local.HeightCell`)) true)
        (else
          (return (struct) false))))))