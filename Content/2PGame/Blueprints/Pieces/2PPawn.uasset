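; Pawn piece for a two-player board game, defining the chess-style moves it can make.
; PotentialMoveList builds candidate cells with GetCellsFromSlide: a forward slide of two cells until the piece has moved, then one, plus two one-cell angled attacks.
; Separate capture modes distinguish the forward move from the attacks.
; The event graph holds only disabled stubs, and no en passant or promotion logic appears here.
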(fn `PotentialMoveList`
  (params (StartCell :type "/Game/2PGame/Blueprints/Board/2PCell Structure"))
  (returns (EndCell :type "Array of /Game/2PGame/Blueprints/Board/2PCell Structure"))
  (locals (Output :type "Array of /Game/2PGame/Blueprints/Board/2PCell Structure"))
  (`|ExecutionSequence`
    (:`then_0`
      (`|ExecutionSequence`
        (:`then_0`
          ;[1 1 1] Move forward 2
          (bind _cellpath (`self.GetCellsFromSlide` (`local.StartCell`) "NewEnumerator0" (select `bool` (`self.HasPieceBeenMoved`) :`false` 2 :`true` 1) "NewEnumerator1"))
          (`KismetArrayLibrary.Array_Append` (`local.Output`) _cellpath))
        (:`then_1`
          ;[1 1 1] Attack (angled)
          (bind _cellpath_2 (`self.GetCellsFromSlide` (`local.StartCell`) "NewEnumerator4" 1 "NewEnumerator2"))
          (`KismetArrayLibrary.Array_Append` (`local.Output`) _cellpath_2)
          (bind _cellpath_3 (`self.GetCellsFromSlide` (`local.StartCell`) "NewEnumerator7" 1 "NewEnumerator2"))
          (`KismetArrayLibrary.Array_Append` (`local.Output`) _cellpath_3))))
    (:`then_1`
      (return (`local.Output`)))))

(fn `UserConstructionScript`
  (`parent.UserConstructionScript`))