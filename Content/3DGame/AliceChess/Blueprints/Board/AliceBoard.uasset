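; Board actor for Alice chess that tracks two side-by-side 8x8 boards in one flat BoardState array.
; BeginPlay spawns both players' pieces on the first board, with helpers converting between cells, array indices and world positions.
; Moves are validated against each piece's PotentialMoveList, then MakeMove teleports the piece, destroys any capture and updates the array.
; SwitchCellDestinationIfValid finds the mirrored cell on the other board by column offset and reports whether it is empty.
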(event `self.ReceiveBeginPlay`
  (if (not true)
    (`/Engine/EditorBlueprintResources/ActorMacros.Switch Has Authority` ; Must Stay Here. Handles replication between client and server
      (:`Authority`
        _)))
  (`KismetArrayLibrary.Array_Resize` (`self.BoardState`) 144)
  (for _index (range 2)
    (`self.MakeKings` _index)
    (`self.MakeQueens` _index)
    (`self.MakeBishops` _index)
    (`self.MakeKnights` _index)
    (`self.MakeRooks` _index)
    (`self.MakePawns` _index)))

(fn `AddPiece`
  (params (Piece :type "/Game/3DGame/AliceChess/Blueprints/Pieces/AlicePiece Object Reference") (Cell :type "/Game/3DGame/AliceChess/Blueprints/Board/AliceCell Structure"))
  (`KismetArrayLibrary.Array_Set` (`self.BoardState`) (`self.GetIndexFromCell` Cell) Piece))

(fn `BoardStateElem`
  (params (`Dimension 1` :type Integer))
  (returns (Output :type "/Game/3DGame/AliceChess/Blueprints/Pieces/AlicePiece Object Reference"))
  (return (`|GetArrayItem` (`self.BoardState`) `Dimension 1`)))

(fn `CellToGrid`
  (params (Cell :type "/Game/3DGame/AliceChess/Blueprints/Board/AliceCell Structure"))
  (returns (ReturnValue :type "Vector Structure"))
  (return (+ (`KismetMathLibrary.MakeVector` (`self.HandleRow` Cell_Row_4_A31AD37F4ABEE7282C2022A30B0EBA3F) (`self.HandleColumn` Cell_Col_2_767D76F24B6395F8CD2202A2E588D57E)) (`self.GridVector`))))

(fn `GetBoardState`
  (returns (BoardState :type "Array of /Game/3DGame/AliceChess/Blueprints/Pieces/AlicePiece Object Reference"))
  (return (`self.BoardState`)))

(fn `GetBoardStateSize`
  (returns (ReturnValue :type Integer))
  (return (`KismetArrayLibrary.Array_Length` (`self.BoardState`))))

(fn `GetCellInfo`
  (params (Cell :type "/Game/3DGame/AliceChess/Blueprints/Board/AliceCell Structure"))
  (returns (TileValid :type Boolean) (TileFree :type Boolean) (BoardPiece :type "/Game/3DGame/AliceChess/Blueprints/Pieces/AlicePiece Object Reference"))
  (bind _piece (`self.PieceAtLocation` (`local.Cell`)))
  (if (`self.IsCellInRange` Cell)
    (return true (not (`KismetSystemLibrary.IsValid` _piece)) _piece)
    (else
      (return false false null))))

(fn `IsCellInRange`
  (params (Cell :type "/Game/3DGame/AliceChess/Blueprints/Board/AliceCell Structure"))
  (returns (InRange :type Boolean))
  (if true
    (return (or (and (`KismetMathLibrary.InRange_IntInt` Cell_Col_2_767D76F24B6395F8CD2202A2E588D57E 0 7) (`KismetMathLibrary.InRange_IntInt` Cell_Row_4_A31AD37F4ABEE7282C2022A30B0EBA3F 0 7)) (and (`KismetMathLibrary.InRange_IntInt` Cell_Col_2_767D76F24B6395F8CD2202A2E588D57E 10 17) (`KismetMathLibrary.InRange_IntInt` Cell_Row_4_A31AD37F4ABEE7282C2022A30B0EBA3F 0 7))))))

(fn `IsMoveAvailable`
  (params (StartCell :type "/Game/3DGame/AliceChess/Blueprints/Board/AliceCell Structure") (EndCell :type "/Game/3DGame/AliceChess/Blueprints/Board/AliceCell Structure"))
  (returns (Result :type Boolean))
  (locals (SelectedPiece :type "/Game/3DGame/AliceChess/Blueprints/Pieces/AlicePiece Object Reference"))
  (bind _output_get (set `local.SelectedPiece` (`self.PieceAtLocation` StartCell)))
  (`/Engine/EditorBlueprintResources/StandardMacros.IsValid` _output_get
    (:`Is Valid`
      (return (`KismetArrayLibrary.Array_Contains` (`/Game/3DGame/AliceChess/Blueprints/Pieces/AlicePiece.PotentialMoveList` (`local.SelectedPiece`) (`local.StartCell`)) (`local.EndCell`))))
    (:`Is Not Valid`
      (return false))))

(fn `MakeBishops`
  (params (`Player Index` :type Integer))
  (locals (Col :type Integer) (Row :type Integer))
  (set `local.Row` (select `int` (`local.Player Index`) :`0` 0 :`1` 7))
  (`|ExecutionSequence`
    (:`then_0`
      (set `local.Col` (select `int` (`local.Player Index`) :`0` 2 :`1` 5))
      (bind _returnvalue (`|SpawnActorFromClass` "/Game/3DGame/AliceChess/Blueprints/Pieces/AliceBishop.AliceBishop_C" (`KismetMathLibrary.MakeTransform` (`self.CellToGrid` (make `/Game/3DGame/AliceChess/Blueprints/Board/AliceCell` (`local.Col`) (`local.Row`)))) "Undefined" "OverrideRootScale" null (`local.Player Index`) null))
      (`self.AddPiece` _returnvalue (make `/Game/3DGame/AliceChess/Blueprints/Board/AliceCell` (`local.Col`) (`local.Row`))))
    (:`then_1`
      (set `local.Col` (select `int` (`local.Player Index`) :`0` 5 :`1` 2))
      (bind _returnvalue_2 (`|SpawnActorFromClass` "/Game/3DGame/AliceChess/Blueprints/Pieces/AliceBishop.AliceBishop_C" (`KismetMathLibrary.MakeTransform` (`self.CellToGrid` (make `/Game/3DGame/AliceChess/Blueprints/Board/AliceCell` (`local.Col`) (`local.Row`)))) "Undefined" "OverrideRootScale" null (`local.Player Index`) null))
      (`self.AddPiece` _returnvalue_2 (make `/Game/3DGame/AliceChess/Blueprints/Board/AliceCell` (`local.Col`) (`local.Row`))))))

(fn `MakeKings`
  (params (`Player Index` :type Integer))
  (locals (Col :type Integer) (Row :type Integer))
  (set `local.Row` (select `int` (`local.Player Index`) :`0` 0 :`1` 7))
  (set `local.Col` 4)
  (bind _returnvalue (`|SpawnActorFromClass` "/Game/3DGame/AliceChess/Blueprints/Pieces/AliceKing.AliceKing_C" (`KismetMathLibrary.MakeTransform` (`self.CellToGrid` (make `/Game/3DGame/AliceChess/Blueprints/Board/AliceCell` (`local.Col`) (`local.Row`)))) "Undefined" "OverrideRootScale" null (`local.Player Index`) null))
  (`self.AddPiece` _returnvalue (make `/Game/3DGame/AliceChess/Blueprints/Board/AliceCell` (`local.Col`) (`local.Row`))))

(fn `MakeKnights`
  (params (PlayerIndex :type Integer))
  (locals (Col :type Integer) (Row :type Integer))
  (set `local.Row` (select `int` (`local.PlayerIndex`) :`0` 0 :`1` 7))
  (`|ExecutionSequence`
    (:`then_0`
      (set `local.Col` (select `int` (`local.PlayerIndex`) :`0` 1 :`1` 6))
      (bind _returnvalue (`|SpawnActorFromClass` "/Game/3DGame/AliceChess/Blueprints/Pieces/AliceKnight.AliceKnight_C" (`KismetMathLibrary.MakeTransform` (`self.CellToGrid` (make `/Game/3DGame/AliceChess/Blueprints/Board/AliceCell` (`local.Col`) (`local.Row`)))) "Undefined" "OverrideRootScale" null (`local.PlayerIndex`) null))
      (`self.AddPiece` _returnvalue (make `/Game/3DGame/AliceChess/Blueprints/Board/AliceCell` (`local.Col`) (`local.Row`))))
    (:`then_1`
      (set `local.Col` (select `int` (`local.PlayerIndex`) :`0` 6 :`1` 1))
      (bind _returnvalue_2 (`|SpawnActorFromClass` "/Game/3DGame/AliceChess/Blueprints/Pieces/AliceKnight.AliceKnight_C" (`KismetMathLibrary.MakeTransform` (`self.CellToGrid` (make `/Game/3DGame/AliceChess/Blueprints/Board/AliceCell` (`local.Col`) (`local.Row`)))) "Undefined" "OverrideRootScale" null (`local.PlayerIndex`) null))
      (`self.AddPiece` _returnvalue_2 (make `/Game/3DGame/AliceChess/Blueprints/Board/AliceCell` (`local.Col`) (`local.Row`))))))

(fn `MakeMove`
  (params (StartCell :type "/Game/3DGame/AliceChess/Blueprints/Board/AliceCell Structure") (EndCell :type "/Game/3DGame/AliceChess/Blueprints/Board/AliceCell Structure"))
  (locals (SelectedPiece :type "/Game/3DGame/AliceChess/Blueprints/Pieces/AlicePiece Object Reference") (EndPiece :type "/Game/3DGame/AliceChess/Blueprints/Pieces/AlicePiece Object Reference"))
  (set `local.SelectedPiece` (`self.PieceAtLocation` StartCell))
  (set `local.EndPiece` (`self.PieceAtLocation` EndCell))
  (`self.K2_SetActorLocation` (`local.SelectedPiece`) (`self.CellToGrid` (`local.EndCell`)) false true)
  (bind _endpiece (`local.EndPiece`)
    (:`then`
      (`self.K2_DestroyActor` _endpiece))
    (:`else`
      _))
  (`self.MovePiece` (`local.StartCell`) (`local.EndCell`)))

(fn `MakePawns`
  (params (PlayerIndex :type Integer))
  (locals (Row :type Integer) (Col :type Integer))
  (set `local.Row` (select `int` (`local.PlayerIndex`) :`0` 1 :`1` 6))
  (for _index (range 8)
    (bind _output_get (set `local.Col` _index))
    (bind _returnvalue (`|SpawnActorFromClass` "/Game/3DGame/AliceChess/Blueprints/Pieces/AlicePawn.AlicePawn_C" (`KismetMathLibrary.MakeTransform` (`self.CellToGrid` (make `/Game/3DGame/AliceChess/Blueprints/Board/AliceCell` _output_get (`local.Row`)))) "Undefined" "OverrideRootScale" null (`local.PlayerIndex`) null))
    (`self.AddPiece` _returnvalue (make `/Game/3DGame/AliceChess/Blueprints/Board/AliceCell` (`local.Col`) (`local.Row`)))))

(fn `MakeQueens`
  (params (`Player Index` :type Integer))
  (locals (Col :type Integer) (Row :type Integer))
  (set `local.Row` (select `int` (`local.Player Index`) :`0` 0 :`1` 7))
  (set `local.Col` 3)
  (bind _returnvalue (`|SpawnActorFromClass` "/Game/3DGame/AliceChess/Blueprints/Pieces/AliceQueen.AliceQueen_C" (`KismetMathLibrary.MakeTransform` (`self.CellToGrid` (make `/Game/3DGame/AliceChess/Blueprints/Board/AliceCell` (`local.Col`) (`local.Row`)))) "Undefined" "OverrideRootScale" null (`local.Player Index`) null))
  (`self.AddPiece` _returnvalue (make `/Game/3DGame/AliceChess/Blueprints/Board/AliceCell` (`local.Col`) (`local.Row`))))

(fn `MakeRooks`
  (params (`Player Index` :type Integer))
  (locals (Col :type Integer) (Row :type Integer))
  (set `local.Row` (select `int` (`local.Player Index`) :`0` 0 :`1` 7))
  (`|ExecutionSequence`
    (:`then_0`
      (set `local.Col` (select `int` (`local.Player Index`) :`0` 0 :`1` 7))
      (bind _returnvalue (`|SpawnActorFromClass` "/Game/3DGame/AliceChess/Blueprints/Pieces/AliceRook.AliceRook_C" (`KismetMathLibrary.MakeTransform` (`self.CellToGrid` (make `/Game/3DGame/AliceChess/Blueprints/Board/AliceCell` (`local.Col`) (`local.Row`)))) "Undefined" "OverrideRootScale" null (`local.Player Index`) null))
      (`self.AddPiece` _returnvalue (make `/Game/3DGame/AliceChess/Blueprints/Board/AliceCell` (`local.Col`) (`local.Row`))))
    (:`then_1`
      (set `local.Col` (select `int` (`local.Player Index`) :`0` 7 :`1` 0))
      (bind _returnvalue_2 (`|SpawnActorFromClass` "/Game/3DGame/AliceChess/Blueprints/Pieces/AliceRook.AliceRook_C" (`KismetMathLibrary.MakeTransform` (`self.CellToGrid` (make `/Game/3DGame/AliceChess/Blueprints/Board/AliceCell` (`local.Col`) (`local.Row`)))) "Undefined" "OverrideRootScale" null (`local.Player Index`) null))
      (`self.AddPiece` _returnvalue_2 (make `/Game/3DGame/AliceChess/Blueprints/Board/AliceCell` (`local.Col`) (`local.Row`))))))

(fn `MovePiece`
  (params (StartCells :type "/Game/3DGame/AliceChess/Blueprints/Board/AliceCell Structure") (EndCells :type "/Game/3DGame/AliceChess/Blueprints/Board/AliceCell Structure"))
  (locals (PieceToMove :type "/Game/3DGame/AliceChess/Blueprints/Pieces/AlicePiece Object Reference"))
  (set `local.PieceToMove` (`self.PieceAtLocation` StartCells))
  (`KismetArrayLibrary.Array_Set` (`self.BoardState`) (`self.GetIndexFromCell` (`local.StartCells`)))
  (`KismetArrayLibrary.Array_Set` (`self.BoardState`) (`self.GetIndexFromCell` (`local.EndCells`)) (`local.PieceToMove`))
  (`/Game/3DGame/AliceChess/Blueprints/Pieces/AlicePiece.WhenMoved` (`local.PieceToMove`)))

(fn `PieceAtLocation`
  (params (Cell :type "/Game/3DGame/AliceChess/Blueprints/Board/AliceCell Structure"))
  (returns (Piece :type "/Game/3DGame/AliceChess/Blueprints/Pieces/AlicePiece Object Reference"))
  (bind _output (`|GetArrayItem` (`self.BoardState`) (`self.GetIndexFromCell` Cell)))
  (`KismetSystemLibrary.PrintString` (`KismetSystemLibrary.GetDisplayName` _output))
  (return _output))

(fn `SwitchCellDestinationIfValid`
  (params (DestinationCell :type "/Game/3DGame/AliceChess/Blueprints/Board/AliceCell Structure"))
  (returns (NewDestinationCell :type "/Game/3DGame/AliceChess/Blueprints/Board/AliceCell Structure") (CellEmpty :type Boolean))
  (locals (TempCell :type "/Game/3DGame/AliceChess/Blueprints/Board/AliceCell Structure"))
  (if (< DestinationCell_Col_2_767D76F24B6395F8CD2202A2E588D57E 8)
    (bind _output_get (set `local.TempCell` (make `/Game/3DGame/AliceChess/Blueprints/Board/AliceCell` (+ DestinationCell_Col_2_767D76F24B6395F8CD2202A2E588D57E 10) DestinationCell_Row_4_A31AD37F4ABEE7282C2022A30B0EBA3F)))
    (bind _output (`self.BoardStateElem` (`self.GetIndexFromCell` (`local.TempCell`))))
    (`/Engine/EditorBlueprintResources/StandardMacros.IsValid` _output
      (:`Is Valid`
        _)
      (:`Is Not Valid`
        (return (`local.TempCell`) true) ; Returns the required cell of the other board and tells us that the cell is empty
      ))
    (else
      (set `local.TempCell` (make `/Game/3DGame/AliceChess/Blueprints/Board/AliceCell` (- DestinationCell_Col_2_767D76F24B6395F8CD2202A2E588D57E 10) DestinationCell_Row_4_A31AD37F4ABEE7282C2022A30B0EBA3F))
      (bind _output_2 (`self.BoardStateElem` (`self.GetIndexFromCell` (`local.TempCell`))))
      (`/Engine/EditorBlueprintResources/StandardMacros.IsValid` _output_2
        (:`Is Valid`
          _)
        (:`Is Not Valid`
          (return (`local.TempCell`) true) ; Returns the required cell of the other board and tells us that the cell is empty
        ))))
  (return (struct) false))

(fn `UserConstructionScript`)

(fn `WorldToGrid`
  (params (WorldLocation :type "Vector Structure"))
  (returns (Cell :type "/Game/3DGame/AliceChess/Blueprints/Board/AliceCell Structure") (InBounds :type Boolean))
  (locals (`Column Cell` :type Integer) (`Row Cell` :type Integer))
  (bind _lengthofcell (`self.LengthOfCell`))
  (bind (_returnvalue_x _returnvalue_y) (`KismetMathLibrary.BreakVector` (- (`local.WorldLocation`) (`self.GridVector`))))
  (`|ExecutionSequence`
    (:`then_0`
      (set `local.Column Cell` (`KismetMathLibrary.FFloor` (/ _returnvalue_y _lengthofcell)))
      (set `local.Row Cell` (`KismetMathLibrary.FFloor` (/ _returnvalue_x _lengthofcell))))
    (:`then_1`
      (if (`self.IsCellInRange` (make `/Game/3DGame/AliceChess/Blueprints/Board/AliceCell` (`local.Column Cell`) (`local.Row Cell`)))
        (return (make `/Game/3DGame/AliceChess/Blueprints/Board/AliceCell` (`local.Column Cell`) (`local.Row Cell`)) true)
        (else
          (return (struct) false))))))