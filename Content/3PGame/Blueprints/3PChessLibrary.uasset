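; Blueprint function library for three-player chess, providing shared lookups for player colors, game state, board and local-mode settings.
; Color helpers map a player index to white, black or blue, with OpponentColor remapping the index first.
; Board access goes through the cast 3P game state, and GetLocalMode reads local mode and player count from the 3P game mode.
; SetLocalMode instead casts to the 2P game mode.
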(fn `Board`
  (returns (Board :type "/Game/3PGame/Blueprints/Board/3PBoard Object Reference"))
  (return (`/Game/3PGame/Blueprints/3PChessGameState.GetBoard` (`self.ChessGameState` (`local.__WorldContext`)))))

(fn `ChessGameState`
  (returns (`Chess Game State` :type "/Game/3PGame/Blueprints/3PChessGameState Object Reference"))
  (return (cast `/Game/3PGame/Blueprints/3PChessGameState` (`GameplayStatics.GetGameState` null) :!pure true)))

(fn `GetLocalMode`
  (returns (`Local Mode` :type Boolean) (PlayerAmount :type Integer))
  (bind (_localmode _playeramount) (`/Game/3PGame/Blueprints/3PChessGameMode.GetLocalMode` (cast `/Game/3PGame/Blueprints/3PChessGameMode` (`GameplayStatics.GetGameMode` (`local.__WorldContext`)) :!pure true)))
  (return _localmode _playeramount))

(fn `OpponentColor`
  (params (PlayerIndex :type Integer))
  (returns (Color :type "LinearColor Structure"))
  (return (`self.PlayerColor` (select `int` PlayerIndex :`0` 2 :`1` 1 :`2` 0) (`local.__WorldContext`))))

(fn `PlayerColor`
  (params (PlayerIndex :type Integer))
  (returns (Color :type "LinearColor Structure"))
  (return (select `int` PlayerIndex :`0` (struct :`R` 0.96875 :`G` 0.972328 :`B` 1.0 :`A` 1.0) :`1` (struct) :`2` (struct :`R` 0.016981 :`B` 1.0 :`A` 1.0) :!type "LinearColor Structure")))

(fn `SetLocalMode`
  (bind (_as2pchess_game_mode _bsuccess) (cast `/Game/2PGame/Blueprints/2PChessGameMode` (`GameplayStatics.GetGameMode` (`local.__WorldContext`)) :!pure true))
  (`KismetSystemLibrary.PrintString` null "Set Local Mode in library")
  (`/Game/2PGame/Blueprints/2PChessGameMode.SetLocalMode` _as2pchess_game_mode _bsuccess))