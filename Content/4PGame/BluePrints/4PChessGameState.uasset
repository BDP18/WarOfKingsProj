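; Game state for four-player chess that holds the board reference and rotates the current turn through the four players.
; Ending a turn advances the player index with wraparound and begins the next turn, which fires OnCurrentPlayerSet; a parallel set of Local turn events mirrors this.
; GetHoveredCell traces from the mouse cursor and converts the hit into a board grid cell.
; The delayed authority-only first-turn start is disconnected, so nothing here begins the first turn.
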(event `self.ReceiveBeginPlay`
  (bind _outactors (`GameplayStatics.GetAllActorsOfClass` "/Game/4PGame/BluePrints/Board/4PBoard.4PBoard_C"))
  (set `self.Board` (`|GetArrayItem` _outactors)))

(event `BeginPlayerTurn`
  (params (PlayerIndex :type Integer))
  (bind _output_get (set `self.CurrentPlayerIndex` PlayerIndex))
  (`self.OnCurrentPlayerSet` _output_get))

(event `EndPlayerTurn`
  (if (== (`self.CurrentPlayerIndex`) 0)
    (set `self.CurrentPlayerIndex` 1)
    (`self.BeginPlayerTurn` (`self.CurrentPlayerIndex`) :!label _label)
    (elif (== (`self.CurrentPlayerIndex`) 1)
      (set `self.CurrentPlayerIndex` 2)
      (goto _label)
      (elif (== (`self.CurrentPlayerIndex`) 2)
        (set `self.CurrentPlayerIndex` 3)
        (goto _label)
        (elif (== (`self.CurrentPlayerIndex`) 3)
          (set `self.CurrentPlayerIndex` 0)
          (goto _label))))))

(event `BeginPlayerTurn(Local)`
  (params (CurrentPlayerIndex :type Integer))
  (bind _output_get (set `self.CurrentPlayerIndex` CurrentPlayerIndex))
  (`self.OnCurrentPlayerSet` _output_get) ; Start Player turn which executes on client and server
  (`KismetSystemLibrary.PrintString` "Begin Player Turn"))

(event `EndPlayerTurn(Local)`
  (if (== (`self.CurrentPlayerIndex`) 0)
    (set `self.CurrentPlayerIndex` 1)
    (`self.BeginPlayerTurn(Local)` (`self.CurrentPlayerIndex`) :!label _label)
    (elif (== (`self.CurrentPlayerIndex`) 1)
      (set `self.CurrentPlayerIndex` 2)
      (goto _label)
      (elif (== (`self.CurrentPlayerIndex`) 2)
        (set `self.CurrentPlayerIndex` 3)
        (goto _label)
        (elif (== (`self.CurrentPlayerIndex`) 3)
          (set `self.CurrentPlayerIndex` 0)
          (goto _label))))))

(fn `Get current Player Index`
  (returns (CurrentPlayerIndex :type Integer))
  (return (`self.CurrentPlayerIndex`)))

(fn `GetBoard`
  (returns (Board :type "/Game/4PGame/BluePrints/Board/4PBoard Object Reference"))
  (return (`self.Board`)))

(fn `GetHoveredCell`
  (params (PlayerController :type "PlayerController Object Reference"))
  (returns (InRange :type Boolean) (Cell :type "/Game/4PGame/BluePrints/Board/4PCell Structure"))
  (bind (_worldlocation _worlddirection) (`PlayerController.DeprojectMousePositionToWorld` PlayerController))
  (bind (_outhit _returnvalue) (`KismetSystemLibrary.LineTraceSingle` _worldlocation (+ _worldlocation (* _worlddirection 10000.0)) "TraceTypeQuery1"))
  (if _returnvalue
    (bind (_cell _inbounds) (`/Game/4PGame/BluePrints/Board/4PBoard.WorldToGrid` (`self.Board`) (`.Location` (`GameplayStatics.BreakHitResult` _outhit))))
    (return _inbounds _cell)
    (else
      (return false))))

(fn `UserConstructionScript`)