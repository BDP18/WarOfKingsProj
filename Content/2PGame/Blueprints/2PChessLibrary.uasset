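; Blueprint function library of shared helpers for a two-player chess game.
; Color helpers map a player index to near-white or near-black, with the opponent's color found by flipping the index.
; World-context lookups return the cast chess game state and its board.
; Local-mode accessors go through the chess game mode: the getter also returns the player amount, and the setter prints a debug string.
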(fn `Board`
  (returns (Board :type "/Game/2PGame/Blueprints/Board/2PBoard Object Reference"))
  (return (`/Game/2PGame/Blueprints/2PChessGameState.GetBoard` (`self.ChessGameState` (`local.__WorldContext`)))))

(fn `ChessGameState`
  (returns (`Chess Game State` :type "/Game/2PGame/Blueprints/2PChessGameState Object Reference"))
  (return (cast `/Game/2PGame/Blueprints/2PChessGameState` (`GameplayStatics.GetGameState` (`local.__WorldContext`)) :!pure true)))

(fn `GetLocalMode`
  (returns (`Local Mode` :type Boolean) (PlayerAmount :type Integer))
  (bind (_localmode _playeramount) (`/Game/2PGame/Blueprints/2PChessGameMode.GetLocalMode` (cast `/Game/2PGame/Blueprints/2PChessGameMode` (`GameplayStatics.GetGameMode` (`local.__WorldContext`)) :!pure true)))
  (return _localmode _playeramount))

(fn `OpponentColor`
  (params (PlayerIndex :type Integer))
  (returns (Color :type "LinearColor Structure"))
  (return (`self.PlayerColor` (select `int` PlayerIndex :`0` 1 :`1` 0) (`local.__WorldContext`))))

(fn `PlayerColor`
  (params (PlayerIndex :type Integer))
  (returns (Color :type "LinearColor Structure"))
  (return (select `int` PlayerIndex :`0` (struct :`R` 0.9 :`G` 0.9 :`B` 0.9 :`A` 1.0) :`1` (struct :`R` 0.01 :`G` 0.01 :`B` 0.01 :`A` 1.0) :!type "LinearColor Structure")))

(fn `SetLocalMode`
  (params (LocalMode :type Boolean))
  (`KismetSystemLibrary.PrintString` null "Set Local Mode in library")
  (bind _as2pchess_game_mode (cast `/Game/2PGame/Blueprints/2PChessGameMode` (`GameplayStatics.GetGameMode` (`local.__WorldContext`))))
  (`/Game/2PGame/Blueprints/2PChessGameMode.SetLocalMode` _as2pchess_game_mode LocalMode))