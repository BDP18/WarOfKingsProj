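; Knight piece for the Millinium 3D chess game, defining which cells it can jump to.
; PotentialMoveList takes a start cell and calls GetCellsFromMove for all 24 two-plus-one L-shaped offsets across the forward, right and up axes.
; A Sequence groups the offsets by plane and direction, appending each result to Output before returning the combined list.
; The event graph and construction script add no logic of their own.
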(fn `PotentialMoveList`
  (params (StartCell :type "/Game/3DGame/Millinium3DChess/BluePrints/Board/MCell Structure"))
  (returns (EndCell :type "Array of /Game/3DGame/Millinium3DChess/BluePrints/Board/MCell Structure"))
  (locals (Output :type "Array of /Game/3DGame/Millinium3DChess/BluePrints/Board/MCell Structure"))
  (`|ExecutionSequence`
    (:`then_0`
      (`|ExecutionSequence`
        (:`then_0`
          (bind _cells (`self.GetCellsFromMove` (`local.StartCell`) 1 2))
          (`KismetArrayLibrary.Array_Append` (`local.Output`) _cells)
          (bind _cells_2 (`self.GetCellsFromMove` (`local.StartCell`) 1 -2))
          (`KismetArrayLibrary.Array_Append` (`local.Output`) _cells_2)
          (bind _cells_3 (`self.GetCellsFromMove` (`local.StartCell`) -1 2))
          (`KismetArrayLibrary.Array_Append` (`local.Output`) _cells_3)
          (bind _cells_4 (`self.GetCellsFromMove` (`local.StartCell`) -1 -2))
          (`KismetArrayLibrary.Array_Append` (`local.Output`) _cells_4))
        (:`then_1`
          (bind _cells_5 (`self.GetCellsFromMove` (`local.StartCell`) 2 1))
          (`KismetArrayLibrary.Array_Append` (`local.Output`) _cells_5)
          (bind _cells_6 (`self.GetCellsFromMove` (`local.StartCell`) 2 -1))
          (`KismetArrayLibrary.Array_Append` (`local.Output`) _cells_6)
          (bind _cells_7 (`self.GetCellsFromMove` (`local.StartCell`) -2 1))
          (`KismetArrayLibrary.Array_Append` (`local.Output`) _cells_7)
          (bind _cells_8 (`self.GetCellsFromMove` (`local.StartCell`) -2 -1))
          (`KismetArrayLibrary.Array_Append` (`local.Output`) _cells_8))
        (:`then_2`
          (bind _cells_9 (`self.GetCellsFromMove` (`local.StartCell`) 0 2 1))
          (`KismetArrayLibrary.Array_Append` (`local.Output`) _cells_9)
          (bind _cells_10 (`self.GetCellsFromMove` (`local.StartCell`) 0 -2 1))
          (`KismetArrayLibrary.Array_Append` (`local.Output`) _cells_10)
          (bind _cells_11 (`self.GetCellsFromMove` (`local.StartCell`) 2 0 1))
          (`KismetArrayLibrary.Array_Append` (`local.Output`) _cells_11)
          (bind _cells_12 (`self.GetCellsFromMove` (`local.StartCell`) -2 0 1))
          (`KismetArrayLibrary.Array_Append` (`local.Output`) _cells_12))
        (:`then_3`
          (bind _cells_13 (`self.GetCellsFromMove` (`local.StartCell`) 0 2 -1))
          (`KismetArrayLibrary.Array_Append` (`local.Output`) _cells_13)
          (bind _cells_14 (`self.GetCellsFromMove` (`local.StartCell`) 0 -2 -1))
          (`KismetArrayLibrary.Array_Append` (`local.Output`) _cells_14)
          (bind _cells_15 (`self.GetCellsFromMove` (`local.StartCell`) 2 0 -1))
          (`KismetArrayLibrary.Array_Append` (`local.Output`) _cells_15)
          (bind _cells_16 (`self.GetCellsFromMove` (`local.StartCell`) -2 0 -1))
          (`KismetArrayLibrary.Array_Append` (`local.Output`) _cells_16))
        (:`then_4`
          (bind _cells_17 (`self.GetCellsFromMove` (`local.StartCell`) 0 1 2))
          (`KismetArrayLibrary.Array_Append` (`local.Output`) _cells_17)
          (bind _cells_18 (`self.GetCellsFromMove` (`local.StartCell`) 0 -1 2))
          (`KismetArrayLibrary.Array_Append` (`local.Output`) _cells_18)
          (bind _cells_19 (`self.GetCellsFromMove` (`local.StartCell`) 1 0 2))
          (`KismetArrayLibrary.Array_Append` (`local.Output`) _cells_19)
          (bind _cells_20 (`self.GetCellsFromMove` (`local.StartCell`) -1 0 2))
          (`KismetArrayLibrary.Array_Append` (`local.Output`) _cells_20))
        (:`then_5`
          (bind _cells_21 (`self.GetCellsFromMove` (`local.StartCell`) 0 1 -2))
          (`KismetArrayLibrary.Array_Append` (`local.Output`) _cells_21)
          (bind _cells_22 (`self.GetCellsFromMove` (`local.StartCell`) 0 -1 -2))
          (`KismetArrayLibrary.Array_Append` (`local.Output`) _cells_22)
          (bind _cells_23 (`self.GetCellsFromMove` (`local.StartCell`) 1 0 -2))
          (`KismetArrayLibrary.Array_Append` (`local.Output`) _cells_23)
          (bind _cells_24 (`self.GetCellsFromMove` (`local.StartCell`) -1 0 -2))
          (`KismetArrayLibrary.Array_Append` (`local.Output`) _cells_24))))
    (:`then_1`
      (return (`local.Output`)))))

(fn `UserConstructionScript`
  (`parent.UserConstructionScript`))