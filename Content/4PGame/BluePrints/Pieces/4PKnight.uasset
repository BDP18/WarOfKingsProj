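; Knight piece Blueprint for the 4P board game, which defines the chess knight's L-shaped movement.
; PotentialMoveList takes a start cell, calls GetCellsFromMove for each of the eight forward/right knight offsets, and returns the appended results as one list.
; It adds no filtering of its own, and the event graph and construction script contain no custom logic.
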(fn `PotentialMoveList`
  (params (StartCell :type "/Game/4PGame/BluePrints/Board/4PCell Structure"))
  (returns (EndCell :type "Array of /Game/4PGame/BluePrints/Board/4PCell Structure"))
  (locals (Output :type "Array of /Game/4PGame/BluePrints/Board/4PCell Structure"))
  (`|ExecutionSequence`
    (:`then_0`
      (`|ExecutionSequence`
        (:`then_0`
          (bind _cells (`self.GetCellsFromMove` (`local.StartCell`) 2 1))
          (`KismetArrayLibrary.Array_Append` (`local.Output`) _cells)
          (bind _cells_2 (`self.GetCellsFromMove` (`local.StartCell`) 2 -1))
          (`KismetArrayLibrary.Array_Append` (`local.Output`) _cells_2))
        (:`then_1`
          (bind _cells_3 (`self.GetCellsFromMove` (`local.StartCell`) -2 1))
          (`KismetArrayLibrary.Array_Append` (`local.Output`) _cells_3)
          (bind _cells_4 (`self.GetCellsFromMove` (`local.StartCell`) -2 -1))
          (`KismetArrayLibrary.Array_Append` (`local.Output`) _cells_4))
        (:`then_2`
          (bind _cells_5 (`self.GetCellsFromMove` (`local.StartCell`) 1 2))
          (`KismetArrayLibrary.Array_Append` (`local.Output`) _cells_5)
          (bind _cells_6 (`self.GetCellsFromMove` (`local.StartCell`) -1 2))
          (`KismetArrayLibrary.Array_Append` (`local.Output`) _cells_6))
        (:`then_3`
          (bind _cells_7 (`self.GetCellsFromMove` (`local.StartCell`) 1 -2))
          (`KismetArrayLibrary.Array_Append` (`local.Output`) _cells_7)
          (bind _cells_8 (`self.GetCellsFromMove` (`local.StartCell`) -1 -2))
          (`KismetArrayLibrary.Array_Append` (`local.Output`) _cells_8))))
    (:`then_1`
      (return (`local.Output`)))))

(fn `UserConstructionScript`
  (`parent.UserConstructionScript`))