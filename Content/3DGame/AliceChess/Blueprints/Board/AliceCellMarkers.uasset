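; AliceCellMarkers draws highlight markers for the hovered and selected board cells in the Alice Chess game.
; The construction script gives each of the two instanced mesh components a dynamic ColorChanger material, green for selected and blue for hovered.
; Setting a cell clears that component's previous instance, then adds a thin scaled instance at the given world location, so only one marker of each type shows.
; Clear functions remove either or both markers.
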(fn `ClearAllCells`
  (`self.ClearHoveredCell`)
  (`self.ClearSelectedCell`))

(fn `ClearHoveredCell`
  (`InstancedStaticMeshComponent.ClearInstances` (`self.HoveredCell`)))

(fn `ClearSelectedCell`
  (`InstancedStaticMeshComponent.ClearInstances` (`self.SelectedCell`)))

(fn `SetHoveredCell`
  (params (Location :type "Vector Structure"))
  (`self.ClearHoveredCell`) ; Clear Previously Hovered Cell
  (`InstancedStaticMeshComponent.AddInstanceWorldSpace` (`self.HoveredCell`) (`KismetMathLibrary.MakeTransform` Location (struct) (0.75 0.75 0.05))))

(fn `SetSelectedCell`
  (params (Location :type "Vector Structure"))
  (`self.ClearSelectedCell`) ; Clear Previously Selected Cell
  (`InstancedStaticMeshComponent.AddInstanceWorldSpace` (`self.SelectedCell`) (`KismetMathLibrary.MakeTransform` Location (struct) (0.75 0.75 0.05))))

(fn `UserConstructionScript`
  (`|ExecutionSequence`
    (:`then_0`
      (bind _returnvalue (`KismetMaterialLibrary.CreateDynamicMaterialInstance` "/Game/Materials/ColorChanger.ColorChanger"))
      (`MaterialInstanceDynamic.SetVectorParameterValue` _returnvalue "Color" (struct :`G` 1.0 :`B` 0.442 :`A` 1.0))
      (`PrimitiveComponent.SetMaterial` (`self.SelectedCell`) 0 _returnvalue))
    (:`then_1`
      (bind _returnvalue_2 (`KismetMaterialLibrary.CreateDynamicMaterialInstance` "/Game/Materials/ColorChanger.ColorChanger"))
      (`MaterialInstanceDynamic.SetVectorParameterValue` _returnvalue_2 "Color" (struct :`B` 1.0 :`A` 1.0))
      (`PrimitiveComponent.SetMaterial` (`self.HoveredCell`) 0 _returnvalue_2))))