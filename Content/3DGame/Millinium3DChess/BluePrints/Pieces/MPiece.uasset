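; Base chess piece for 3D chess: sets player color and facing, turns blue on hover, and tracks moved and en passant state.
; PotentialMoveList is an empty stub, presumably for child pieces, alongside single-step and sliding cell-list helpers.
; Both offset cells in three axes, mirrored per player, then query the Board through CanPieceMoveToCell for validity, occupancy and capture mode.
; GetDirections holds unconnected tables for 3D directions.
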(event `self.ReceiveBeginPlay`
  (bind _returnvalue (`KismetMaterialLibrary.CreateDynamicMaterialInstance` "/Game/Boardgame_Collection/Materials/Realistic/MI_White.MI_White"))
  (`PrimitiveComponent.SetMaterial` (`self.StaticMesh`) 0 _returnvalue)
  (`MaterialInstanceDynamic.SetVectorParameterValue` _returnvalue "Color" (`/Game/2PGame/Blueprints/2PChessLibrary.PlayerColor` (`self.CurrentPlayerIndex`)))
  (if (== (`self.CurrentPlayerIndex`) 1)
    (`self.K2_SetActorRotation` (struct :`Yaw` -90.0))
    (else
      (`self.K2_SetActorRotation` (struct :`Yaw` 90.0)))))

(event `WhenMoved`
  (set `self.HasBeenMoved` true))

(event `self.StaticMesh.OnBeginCursorOver`
  (params (TouchedComponent :type "PrimitiveComponent Object Reference"))
  (`self.EnableInput` (`GameplayStatics.GetPlayerController` (`self.CurrentPlayerIndex`)))
  (bind _returnvalue (`PrimitiveComponent.CreateDynamicMaterialInstance` (`self.StaticMesh`) 0 "/Game/2PGame/Blueprints/Materials/M_TileHighlight.M_TileHighlight" "None"))
  (`MaterialInstanceDynamic.SetVectorParameterValue` _returnvalue "Color" (struct :`B` 1.0 :`A` 1.0))
  (`PrimitiveComponent.SetMaterial` (`self.StaticMesh`) 0 _returnvalue))

(fn `CanPieceMoveToCell`
  (params (Cell :type "/Game/3DGame/Millinium3DChess/BluePrints/Board/MCell Structure") (CaptureMode :type "/Game/3DGame/Millinium3DChess/BluePrints/MCaptureMode Enum" :default "NewEnumerator0"))
  (returns (Result :type Boolean) (LastInLine :type Boolean))
  (locals (`LastInLine (local)` :type Boolean) (`Add (local)` :type Boolean))
  (`|ExecutionSequence`
    (:`then_0`
      (bind (_tilevalid _tilefree _boardpiece) (`/Game/3DGame/Millinium3DChess/BluePrints/Board/MBoard.GetCellInfo` (`/Game/3DGame/Millinium3DChess/BluePrints/MChessLibrary.Board`) (`local.Cell`)))
      (if _tilevalid
        (if _tilefree
          (if (`|EnumEquality` (`local.CaptureMode`) "NewEnumerator2")
            (set `local.LastInLine (local)` true)
            (else
              (set `local.Add (local)` true :!label _label)))
          (else
            (set `local.LastInLine (local)` true)
            (if (and (`|EnumInequality` (`local.CaptureMode`) "NewEnumerator1") (!= (`/Game/3DGame/Millinium3DChess/BluePrints/Pieces/MPiece.CurrentPlayerIndex` _boardpiece) (`self.CurrentPlayerIndex`)))
              (goto _label))))
        (else
          (set `local.LastInLine (local)` true))))
    (:`then_1`
      (return (`local.Add (local)`) (`local.LastInLine (local)`)))))

(fn `CellAfterMoved`
  (params (Cell :type "/Game/3DGame/Millinium3DChess/BluePrints/Board/MCell Structure") (Forward :type Integer :default 1) (Right :type Integer) (Up :type Integer))
  (returns (NewCell :type "/Game/3DGame/Millinium3DChess/BluePrints/Board/MCell Structure"))
  (bind (_x _y _z) (break `/Game/3DGame/Millinium3DChess/BluePrints/Board/MCell` (`local.Cell`)))
  (bind _returnvalue (select `int` (`self.CurrentPlayerIndex`) :`0` 1 :`1` -1))
  (`KismetSystemLibrary.PrintString` "TestCell")
  (`KismetSystemLibrary.PrintString` (`KismetStringLibrary.Conv_IntVectorToString` (make `IntVector` _x _y _z)))
  (return (make `/Game/3DGame/Millinium3DChess/BluePrints/Board/MCell` (+ Cell_X_7_767D76F24B6395F8CD2202A2E588D57E (* (`local.Forward`) _returnvalue)) (+ Cell_Y_8_A31AD37F4ABEE7282C2022A30B0EBA3F (* _returnvalue (`local.Right`))) (+ Cell_Z_9_A0ABD97541C337FF31685EB1A05A7A38 Up))))

(fn `GetCellsFromMove`
  (params (Cell :type "/Game/3DGame/Millinium3DChess/BluePrints/Board/MCell Structure") (Forward :type Integer) (Right :type Integer) (Up :type Integer) (CaptureMode :type "/Game/3DGame/Millinium3DChess/BluePrints/MCaptureMode Enum" :default "NewEnumerator0"))
  (returns (Cells :type "Array of /Game/3DGame/Millinium3DChess/BluePrints/Board/MCell Structure"))
  (locals (CurrentCell :type "/Game/3DGame/Millinium3DChess/BluePrints/Board/MCell Structure"))
  (bind _newcell (`self.CellAfterMoved` Cell Forward Right Up))
  (bind _output_get (set `local.CurrentCell` _newcell))
  (bind _result (`self.CanPieceMoveToCell` _output_get (`local.CaptureMode`)))
  (if _result
    (return (`|MakeArray` (`local.CurrentCell`)))
    (else
      (return))))

(fn `GetCellsFromSlide`
  (params (Cell :type "/Game/3DGame/Millinium3DChess/BluePrints/Board/MCell Structure") (Direction :type "/Game/3DGame/Millinium3DChess/BluePrints/MMoveDirection Enum" :default "NewEnumerator0") (MaxDistance :type Integer) (Capture :type "/Game/3DGame/Millinium3DChess/BluePrints/MCaptureMode Enum" :default "NewEnumerator0"))
  (returns (CellPath :type "Array of /Game/3DGame/Millinium3DChess/BluePrints/Board/MCell Structure"))
  (locals (CurrentCell :type "/Game/3DGame/Millinium3DChess/BluePrints/Board/MCell Structure") (Loop :type Boolean :default true) (Output :type "Array of /Game/3DGame/Millinium3DChess/BluePrints/Board/MCell Structure") (Distance :type Integer))
  (bind (_right _forward _up) (`self.GetDirections` (`local.Direction`) (`local.Direction`) (`local.Direction`)))
  (set `local.CurrentCell` Cell)
  (while (and (`local.Loop`) (< (`local.Distance`) (`local.MaxDistance`)))
    (`/Engine/EditorBlueprintResources/StandardMacros.IncrementInt` (`local.Distance`)
      (:`  `
        (bind _newcell (`self.CellAfterMoved` (`local.CurrentCell`) _right _forward _up))
        (bind _output_get (set `local.CurrentCell` _newcell))
        (bind (_result _lastinline) (`self.CanPieceMoveToCell` _output_get (`local.Capture`)))
        (set `local.Loop` (not _lastinline))
        (if _result
          (`KismetArrayLibrary.Array_Add` (`local.Output`) (`local.CurrentCell`))))))
  (return (`local.Output`)))

(fn `HasPieceBeenMoved`
  (returns (HasBeenMoved :type Boolean))
  (return (`self.HasBeenMoved`)))

(fn `PotentialMoveList`
  (params (StartCell :type "/Game/3DGame/Millinium3DChess/BluePrints/Board/MCell Structure"))
  (returns (EndCell :type "Array of /Game/3DGame/Millinium3DChess/BluePrints/Board/MCell Structure"))
  (return))

(fn `ResetEnPassantVulnerable`
  (set `self.EnPassantVulnerable` false))

(fn `SetEnPassantVulnerable`
  (set `self.EnPassantVulnerable` true))

(fn `UserConstructionScript`)