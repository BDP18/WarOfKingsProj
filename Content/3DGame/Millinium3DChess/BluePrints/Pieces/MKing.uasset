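; King piece for Millinium 3D Chess, defining which cells the king can potentially move to.
; PotentialMoveList calls GetCellsFromSlide with a max distance of one for each of 26 directions, covering every neighboring cell in three dimensions.
; Each result is appended to a single output list, which is returned after all directions are gathered.
; The event graph is unused, and the construction script only calls its parent.
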(fn `PotentialMoveList`
  (params (StartCell :type "/Game/3DGame/Millinium3DChess/BluePrints/Board/MCell Structure"))
  (returns (EndCell :type "Array of /Game/3DGame/Millinium3DChess/BluePrints/Board/MCell Structure"))
  (locals (Output :type "Array of /Game/3DGame/Millinium3DChess/BluePrints/Board/MCell Structure"))
  (`|ExecutionSequence`
    (:`then_0`
      (`|ExecutionSequence`
        (:`then_0`
          (bind _cellpath (`self.GetCellsFromSlide` (`local.StartCell`) "NewEnumerator0" 1))
          (`KismetArrayLibrary.Array_Append` (`local.Output`) _cellpath)
          (bind _cellpath_2 (`self.GetCellsFromSlide` (`local.StartCell`) "NewEnumerator11" 1))
          (`KismetArrayLibrary.Array_Append` (`local.Output`) _cellpath_2))
        (:`then_1`
          (bind _cellpath_3 (`self.GetCellsFromSlide` (`local.StartCell`) "NewEnumerator4" 1))
          (`KismetArrayLibrary.Array_Append` (`local.Output`) _cellpath_3)
          (bind _cellpath_4 (`self.GetCellsFromSlide` (`local.StartCell`) "NewEnumerator12" 1))
          (`KismetArrayLibrary.Array_Append` (`local.Output`) _cellpath_4)
          (bind _cellpath_5 (`self.GetCellsFromSlide` (`local.StartCell`) "NewEnumerator22" 1))
          (`KismetArrayLibrary.Array_Append` (`local.Output`) _cellpath_5))
        (:`then_2`
          (bind _cellpath_6 (`self.GetCellsFromSlide` (`local.StartCell`) "NewEnumerator3" 1))
          (`KismetArrayLibrary.Array_Append` (`local.Output`) _cellpath_6)
          (bind _cellpath_7 (`self.GetCellsFromSlide` (`local.StartCell`) "NewEnumerator13" 1))
          (`KismetArrayLibrary.Array_Append` (`local.Output`) _cellpath_7)
          (bind _cellpath_8 (`self.GetCellsFromSlide` (`local.StartCell`) "NewEnumerator23" 1))
          (`KismetArrayLibrary.Array_Append` (`local.Output`) _cellpath_8))
        (:`then_3`
          (bind _cellpath_9 (`self.GetCellsFromSlide` (`local.StartCell`) "NewEnumerator1" 1))
          (`KismetArrayLibrary.Array_Append` (`local.Output`) _cellpath_9)
          (bind _cellpath_10 (`self.GetCellsFromSlide` (`local.StartCell`) "NewEnumerator14" 1))
          (`KismetArrayLibrary.Array_Append` (`local.Output`) _cellpath_10))
        (:`then_4`
          (bind _cellpath_11 (`self.GetCellsFromSlide` (`local.StartCell`) "NewEnumerator2" 1))
          (`KismetArrayLibrary.Array_Append` (`local.Output`) _cellpath_11)
          (bind _cellpath_12 (`self.GetCellsFromSlide` (`local.StartCell`) "NewEnumerator15" 1))
          (`KismetArrayLibrary.Array_Append` (`local.Output`) _cellpath_12))
        (:`then_5`
          (bind _cellpath_13 (`self.GetCellsFromSlide` (`local.StartCell`) "NewEnumerator5" 1))
          (`KismetArrayLibrary.Array_Append` (`local.Output`) _cellpath_13)
          (bind _cellpath_14 (`self.GetCellsFromSlide` (`local.StartCell`) "NewEnumerator25" 1))
          (`KismetArrayLibrary.Array_Append` (`local.Output`) _cellpath_14))
        (:`then_6`
          (bind _cellpath_15 (`self.GetCellsFromSlide` (`local.StartCell`) "NewEnumerator6" 1))
          (`KismetArrayLibrary.Array_Append` (`local.Output`) _cellpath_15)
          (bind _cellpath_16 (`self.GetCellsFromSlide` (`local.StartCell`) "NewEnumerator16" 1))
          (`KismetArrayLibrary.Array_Append` (`local.Output`) _cellpath_16))
        (:`then_7`
          (bind _cellpath_17 (`self.GetCellsFromSlide` (`local.StartCell`) "NewEnumerator7" 1))
          (`KismetArrayLibrary.Array_Append` (`local.Output`) _cellpath_17)
          (bind _cellpath_18 (`self.GetCellsFromSlide` (`local.StartCell`) "NewEnumerator17" 1))
          (`KismetArrayLibrary.Array_Append` (`local.Output`) _cellpath_18))
        (:`then_8`
          (bind _cellpath_19 (`self.GetCellsFromSlide` (`local.StartCell`) "NewEnumerator24" 1))
          (`KismetArrayLibrary.Array_Append` (`local.Output`) _cellpath_19)
          (bind _cellpath_20 (`self.GetCellsFromSlide` (`local.StartCell`) "NewEnumerator18" 1))
          (`KismetArrayLibrary.Array_Append` (`local.Output`) _cellpath_20))
        (:`then_9`
          (bind _cellpath_21 (`self.GetCellsFromSlide` (`local.StartCell`) "NewEnumerator8" 1))
          (`KismetArrayLibrary.Array_Append` (`local.Output`) _cellpath_21)
          (bind _cellpath_22 (`self.GetCellsFromSlide` (`local.StartCell`) "NewEnumerator19" 1))
          (`KismetArrayLibrary.Array_Append` (`local.Output`) _cellpath_22))
        (:`then_10`
          (bind _cellpath_23 (`self.GetCellsFromSlide` (`local.StartCell`) "NewEnumerator9" 1))
          (`KismetArrayLibrary.Array_Append` (`local.Output`) _cellpath_23)
          (bind _cellpath_24 (`self.GetCellsFromSlide` (`local.StartCell`) "NewEnumerator20" 1))
          (`KismetArrayLibrary.Array_Append` (`local.Output`) _cellpath_24))
        (:`then_11`
          (bind _cellpath_25 (`self.GetCellsFromSlide` (`local.StartCell`) "NewEnumerator10" 1))
          (`KismetArrayLibrary.Array_Append` (`local.Output`) _cellpath_25)
          (bind _cellpath_26 (`self.GetCellsFromSlide` (`local.StartCell`) "NewEnumerator21" 1))
          (`KismetArrayLibrary.Array_Append` (`local.Output`) _cellpath_26))))
    (:`then_1`
      (return (`local.Output`)))))

(fn `UserConstructionScript`
  (`parent.UserConstructionScript`))