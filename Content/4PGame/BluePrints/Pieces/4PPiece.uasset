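; Base piece for a four-player board game, with an empty PotentialMoveList stub and a flag for whether it has moved.
; On BeginPlay it tints a dynamic material with the player's color and rotates to that player's orientation.
; CellAfterMove maps forward/right offsets into board coordinates per player, feeding slide and single-step helpers.
; CanPieceMoveToCell filters cells by board validity, occupancy, owner and capture mode, and ends blocked slides.
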(event `self.ReceiveBeginPlay`
  (bind _returnvalue (`KismetMaterialLibrary.CreateDynamicMaterialInstance` "/Game/Boardgame_Collection/Materials/M_Piece.M_Piece"))
  (`PrimitiveComponent.SetMaterial` (`self.StaticMesh`) 0 _returnvalue)
  (`MaterialInstanceDynamic.SetVectorParameterValue` _returnvalue "Color" (`/Game/4PGame/BluePrints/4PChessLibrary.PlayerColor` (`self.CurrentPlayerIndex`)))
  (if (== (`self.CurrentPlayerIndex`) 1)
    (`self.K2_SetActorRotation` (struct :`Yaw` 180.0))
    (elif (== (`self.CurrentPlayerIndex`) 2)
      (`self.K2_SetActorRotation` (struct :`Yaw` 90.0))
      (elif (== (`self.CurrentPlayerIndex`) 3)
        (`self.K2_SetActorRotation` (struct :`Yaw` 270.0))))))

(event `WhenMoved`
  (set `self.HasBeenMoved` true))

(fn `CanPieceMoveToCell`
  (params (Cell :type "/Game/4PGame/BluePrints/Board/4PCell Structure") (CaptureMode :type "/Game/4PGame/BluePrints/4PCaptureMode Enum" :default "NewEnumerator0"))
  (returns (Result :type Boolean) (LastInLine :type Boolean))
  (locals (`LastInLine (local)` :type Boolean) (`Add (local)` :type Boolean))
  (`|ExecutionSequence`
    (:`then_0`
      (bind (_cellisvalid _cellisfree _boardpiece) (`/Game/4PGame/BluePrints/Board/4PBoard.GetCellInfo` (`/Game/4PGame/BluePrints/4PChessLibrary.Board`) (`local.Cell`)))
      (if _cellisvalid
        (if _cellisfree
          (if (`|EnumEquality` (`local.CaptureMode`) "NewEnumerator2")
            (set `local.LastInLine (local)` true)
            (else
              (set `local.Add (local)` true :!label _label)))
          (else
            (set `local.LastInLine (local)` true)
            (if (and (`|EnumInequality` (`local.CaptureMode`) "NewEnumerator1") (!= (`/Game/4PGame/BluePrints/Pieces/4PPiece.CurrentPlayerIndex` _boardpiece) (`self.CurrentPlayerIndex`)))
              (goto _label))))
        (else
          (set `local.LastInLine (local)` true))))
    (:`then_1`
      (return (`local.Add (local)`) (`local.LastInLine (local)`)))))

(fn `CellAfterMove`
  (params (Cell :type "/Game/4PGame/BluePrints/Board/4PCell Structure") (Forward :type Integer :default 1) (Right :type Integer))
  (returns (EndCell :type "/Game/4PGame/BluePrints/Board/4PCell Structure"))
  (bind _currentplayerindex (`self.CurrentPlayerIndex`))
  (bind _returnvalue (select `int` (`self.CurrentPlayerIndex`) :`0` 0 :`1` -1 :`2` 0 :`3` 1))
  (bind _returnvalue_2 (select `int` (`self.CurrentPlayerIndex`) :`0` 1 :`1` 0 :`2` -1 :`3` 0))
  (bind _returnvalue_3 (+ Cell_Row_4_A31AD37F4ABEE7282C2022A30B0EBA3F (* _returnvalue_2 (`local.Forward`))))
  (bind _returnvalue_4 (+ Cell_Col_2_767D76F24B6395F8CD2202A2E588D57E (* (`local.Right`) _returnvalue_2)))
  (bind _returnvalue_5 (+ Cell_Row_4_A31AD37F4ABEE7282C2022A30B0EBA3F (* (`local.Right`) _returnvalue)))
  (bind _returnvalue_6 (+ Cell_Col_2_767D76F24B6395F8CD2202A2E588D57E (* _returnvalue (`local.Forward`))))
  (if (== _currentplayerindex 0)
    (`KismetSystemLibrary.PrintString` "Cell expected")
    (`KismetSystemLibrary.PrintString` (`KismetStringLibrary.Conv_IntToString` _returnvalue_4))
    (`KismetSystemLibrary.PrintString` (`KismetStringLibrary.Conv_IntToString` _returnvalue_3))
    (elif (== _currentplayerindex 2)
      _
      (else
        (`KismetSystemLibrary.PrintString` "Cell expected")
        (`KismetSystemLibrary.PrintString` (`KismetStringLibrary.Conv_IntToString` _returnvalue_6))
        (`KismetSystemLibrary.PrintString` (`KismetStringLibrary.Conv_IntToString` _returnvalue_5))
        (return (make `/Game/4PGame/BluePrints/Board/4PCell` _returnvalue_6 _returnvalue_5)))))
  (return (make `/Game/4PGame/BluePrints/Board/4PCell` _returnvalue_4 _returnvalue_3)))

(fn `GetCellsFromMove`
  (params (Cell :type "/Game/4PGame/BluePrints/Board/4PCell Structure") (Forward :type Integer) (Right :type Integer) (CaptureMode :type "/Game/4PGame/BluePrints/4PCaptureMode Enum" :default "NewEnumerator0"))
  (returns (Cells :type "Array of /Game/4PGame/BluePrints/Board/4PCell Structure"))
  (locals (CurrentCell :type "/Game/4PGame/BluePrints/Board/4PCell Structure"))
  (bind _endcell (`self.CellAfterMove` Cell Forward Right))
  (bind _output_get (set `local.CurrentCell` _endcell))
  (bind _result (`self.CanPieceMoveToCell` _output_get (`local.CaptureMode`)))
  (if _result
    (return (`|MakeArray` (`local.CurrentCell`)))
    (else
      (return))))

(fn `GetCellsFromSlide`
  (params (Cell :type "/Game/4PGame/BluePrints/Board/4PCell Structure") (Direction :type "/Game/4PGame/BluePrints/4PMovement Enum" :default "NewEnumerator0") (MaxDistance :type Integer) (CaptureMode :type "/Game/4PGame/BluePrints/4PCaptureMode Enum" :default "NewEnumerator0"))
  (returns (CellPath :type "Array of /Game/4PGame/BluePrints/Board/4PCell Structure"))
  (locals (CurrentCell :type "/Game/4PGame/BluePrints/Board/4PCell Structure") (Loop :type Boolean :default true) (Output :type "Array of /Game/4PGame/BluePrints/Board/4PCell Structure") (Distance :type Integer))
  (set `local.CurrentCell` Cell)
  (while (and (`local.Loop`) (< (`local.Distance`) (`local.MaxDistance`)))
    (`/Engine/EditorBlueprintResources/StandardMacros.IncrementInt` (`local.Distance`)
      (:`  `
        (bind _endcell (`self.CellAfterMove` (`local.CurrentCell`) (select `/Game/4PGame/BluePrints/4PMovement` (`local.Direction`) :`NewEnumerator0` 1 :`NewEnumerator4` 1 :`NewEnumerator1` -1 :`NewEnumerator2` -1 :`NewEnumerator5` -1 :`NewEnumerator7` 1) (select `/Game/4PGame/BluePrints/4PMovement` (`local.Direction`) :`NewEnumerator4` 1 :`NewEnumerator3` 1 :`NewEnumerator1` 1 :`NewEnumerator5` -1 :`NewEnumerator6` -1 :`NewEnumerator7` -1))) ; Changes direction of piece movement according to player index
        (bind _output_get (set `local.CurrentCell` _endcell))
        (bind (_result _lastinline) (`self.CanPieceMoveToCell` _output_get (`local.CaptureMode`)))
        (set `local.Loop` (not _lastinline))
        (if _result
          (`KismetArrayLibrary.Array_Add` (`local.Output`) (`local.CurrentCell`))))))
  (return (`local.Output`)))

(fn `HasPieceBeenMoved`
  (returns (HasBeenMoved :type Boolean))
  (return (`self.HasBeenMoved`)))

(fn `PotentialMoveList`
  (params (StartCell :type "/Game/4PGame/BluePrints/Board/4PCell Structure"))
  (returns (EndCell :type "Array of /Game/4PGame/BluePrints/Board/4PCell Structure"))
  (return))

(fn `UserConstructionScript`)