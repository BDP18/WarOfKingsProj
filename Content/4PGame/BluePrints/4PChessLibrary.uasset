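; Blueprint function library of shared helpers for a four-player chess game.
; PlayerColor maps player indices to white, black, blue and green, and OpponentColor reuses it with fixed pairings (0↔3, 1↔2).
; Shortcuts cast to the 4PChess game state to reach the board, and to the game mode to read local mode with player count or set local mode, printing a debug message on set.
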(fn `Board`
  (returns (Board :type "/Game/4PGame/BluePrints/Board/4PBoard Object Reference"))
  (return (`/Game/4PGame/BluePrints/4PChessGameState.GetBoard` (`self.ChessGameState` (`local.__WorldContext`)))))

(fn `ChessGameState`
  (returns (`Chess Game State` :type "/Game/4PGame/BluePrints/4PChessGameState Object Reference"))
  (return (cast `/Game/4PGame/BluePrints/4PChessGameState` (`GameplayStatics.GetGameState` null) :!pure true)))

(fn `GetLocalMode`
  (returns (`Local Mode` :type Boolean) (PlayerAmount :type Integer))
  (bind (_local_mode _playeramount) (`self.GetLocalMode` (cast `/Game/4PGame/BluePrints/4PChessGameMode` (`GameplayStatics.GetGameMode` (`local.__WorldContext`)) :!pure true)))
  (return _local_mode _playeramount))

(fn `OpponentColor`
  (params (PlayerIndex :type Integer))
  (returns (Color :type "LinearColor Structure"))
  (return (`self.PlayerColor` (select `int` PlayerIndex :`0` 3 :`1` 2 :`2` 1 :`3` 0) (`local.__WorldContext`))))

(fn `PlayerColor`
  (params (PlayerIndex :type Integer))
  (returns (Color :type "LinearColor Structure"))
  (return (select `int` PlayerIndex :`0` (struct :`R` 0.9 :`G` 0.9 :`B` 0.9 :`A` 1.0) :`1` (struct :`R` 0.01 :`G` 0.01 :`B` 0.01 :`A` 1.0) :`2` (struct :`G` 0.014029 :`B` 1.0 :`A` 1.0) :`3` (struct :`G` 1.0 :`B` 0.104131 :`A` 1.0) :!type "LinearColor Structure")))

(fn `SetLocalMode`
  (params (IsLocalGame :type Boolean) (IsLocalGame1 :type Boolean))
  (`KismetSystemLibrary.PrintString` null "Set Local Mode in library")
  (`/Game/4PGame/BluePrints/4PChessGameMode.SetLocalMode` (cast `/Game/4PGame/BluePrints/4PChessGameMode` (`GameplayStatics.GetGameMode` (`local.__WorldContext`)) :!pure true) IsLocalGame1))