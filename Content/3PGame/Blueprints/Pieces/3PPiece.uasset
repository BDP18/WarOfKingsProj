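; Base piece for a three-player board game, tinted and rotated for its owning player, tracking whether it has moved.
; Slide and single-step helpers build candidate cells on three-axis coordinates, checking board validity, occupancy and capture mode.
; PotentialMoveList is an empty stub.
; CellAfterMove maps offsets only for player 0, reusing the Y offset for Z, and returns zero for other players.
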(event `self.ReceiveBeginPlay`
  (bind _returnvalue (`KismetMaterialLibrary.CreateDynamicMaterialInstance` "/Game/Boardgame_Collection/Materials/M_Piece.M_Piece"))
  (`PrimitiveComponent.SetMaterial` (`self.StaticMesh`) 0 _returnvalue)
  (`MaterialInstanceDynamic.SetVectorParameterValue` _returnvalue "Color" (`/Game/3PGame/Blueprints/3PChessLibrary.PlayerColor` (`self.CurrentPlayerIndex`)))
  (if (== (`self.CurrentPlayerIndex`) 0)
    (`self.K2_SetActorRotation` (struct :`Yaw` 180.0))
    (elif (== (`self.CurrentPlayerIndex`) 1)
      (`self.K2_SetActorRotation` (struct :`Yaw` 90.0))
      (elif (== (`self.CurrentPlayerIndex`) 2)
        (`self.K2_SetActorRotation` (struct :`Yaw` 270.0))))))

(event `WhenMoved`
  (set `self.HasBeenMoved` true))

(fn `CanPieceMoveToCell`
  (params (Cell :type "/Game/3PGame/Blueprints/Board/3PCell Structure") (CaptureMode :type "/Game/3PGame/Blueprints/3PCaptureMode Enum" :default "NewEnumerator0"))
  (returns (Result :type Boolean) (LastInLine :type Boolean))
  (locals (`LastInLine (local)` :type Boolean) (`Add (local)` :type Boolean))
  (`|ExecutionSequence`
    (:`then_0`
      (bind (_cellisvalid _cellisfree _boardpiece) (`/Game/3PGame/Blueprints/Board/3PBoard.GetCellInfo` (`/Game/3PGame/Blueprints/3PChessLibrary.Board`) (`local.Cell`)))
      (if _cellisvalid
        (if _cellisfree
          (if (`|EnumEquality` (`local.CaptureMode`) "NewEnumerator0")
            (set `local.LastInLine (local)` true)
            (else
              (set `local.Add (local)` true :!label _label)))
          (else
            (set `local.LastInLine (local)` true)
            (if (and (`|EnumInequality` (`local.CaptureMode`) "NewEnumerator1") (!= (`/Game/3PGame/Blueprints/Pieces/3PPiece.CurrentPlayerIndex` _boardpiece) (`self.CurrentPlayerIndex`)))
              (goto _label))))
        (else
          (set `local.LastInLine (local)` true))))
    (:`then_1`
      (return (`local.Add (local)`) (`local.LastInLine (local)`)))))

(fn `CellAfterMove`
  (params (Cell :type "/Game/3PGame/Blueprints/Board/3PCell Structure") (LocationX :type Integer :default 1) (LocationY :type Integer) (LocationZ :type Integer))
  (returns (EndCell :type "/Game/3PGame/Blueprints/Board/3PCell Structure"))
  (bind _returnvalue (select `int` (`self.CurrentPlayerIndex`) :`0` 1 :`1` -1 :`2` 1))
  (if (== (`self.CurrentPlayerIndex`) 0)
    (return (make `/Game/3PGame/Blueprints/Board/3PCell` (+ Cell_X_9_8F3EF96F4DE7CFA99285238BAEB30378 (* (`local.LocationX`) _returnvalue)) (+ Cell_Y_10_538F45774E13D1994DCBCE9D58BA3D0D (* _returnvalue (`local.LocationY`))) (+ (* _returnvalue (`local.LocationY`)) Cell_Z_12_9475A3A648FE32F9EBEF1CB0BDC294F0)))
    (elif (== (`self.CurrentPlayerIndex`) 1)
      (return (make `/Game/3PGame/Blueprints/Board/3PCell` 0))
      (else
        (return (make `/Game/3PGame/Blueprints/Board/3PCell` 0))))))

(fn `GetCellsFromMove`
  (params (Cell :type "/Game/3PGame/Blueprints/Board/3PCell Structure") (`x+` :type Integer) (`Y+` :type Integer) (`Z+` :type Integer) (CaptureMode :type "/Game/3PGame/Blueprints/3PCaptureMode Enum" :default "NewEnumerator0"))
  (returns (Cells :type "Array of /Game/3PGame/Blueprints/Board/3PCell Structure"))
  (locals (CurrentCell :type "/Game/3PGame/Blueprints/Board/3PCell Structure"))
  (bind _endcell (`self.CellAfterMove` Cell `x+` `Y+` `Z+`))
  (bind _output_get (set `local.CurrentCell` _endcell))
  (bind _result (`self.CanPieceMoveToCell` _output_get (`local.CaptureMode`)))
  (if _result
    (return (`|MakeArray` (`local.CurrentCell`)))
    (else
      (return))))

(fn `GetCellsFromSlide`
  (params (Cell :type "/Game/3PGame/Blueprints/Board/3PCell Structure") (Direction :type "/Game/3PGame/Blueprints/3PMovement Enum" :default "NewEnumerator0") (MaxDistance :type Integer) (CaptureMode :type "/Game/3PGame/Blueprints/3PCaptureMode Enum" :default "NewEnumerator0"))
  (returns (CellPath :type "Array of /Game/3PGame/Blueprints/Board/3PCell Structure"))
  (locals (CurrentCell :type "/Game/3PGame/Blueprints/Board/3PCell Structure") (Loop :type Boolean :default true) (Output :type "Array of /Game/3PGame/Blueprints/Board/3PCell Structure") (Distance :type Integer))
  (set `local.CurrentCell` Cell)
  (while (and (`local.Loop`) (< (`local.Distance`) (`local.MaxDistance`)))
    (`/Engine/EditorBlueprintResources/StandardMacros.IncrementInt` (`local.Distance`)
      (:`  `
        (bind _endcell (`self.CellAfterMove` (`local.CurrentCell`) (select `/Game/3PGame/Blueprints/3PMovement` (`local.Direction`) :`NewEnumerator0` 1 :`NewEnumerator4` 1 :`NewEnumerator3` 1 :`NewEnumerator2` -1 :`NewEnumerator5` -1 :`NewEnumerator6` -1) (select `/Game/3PGame/Blueprints/3PMovement` (`local.Direction`) :`NewEnumerator0` 1 :`NewEnumerator3` -1 :`NewEnumerator1` -1 :`NewEnumerator2` -1 :`NewEnumerator6` 1 :`NewEnumerator7` 1) (select `/Game/3PGame/Blueprints/3PMovement` (`local.Direction`) :`NewEnumerator0` -2 :`NewEnumerator4` -1 :`NewEnumerator1` 1 :`NewEnumerator5` 1 :`NewEnumerator7` -1)))
        (bind _output_get (set `local.CurrentCell` _endcell))
        (bind (_result _lastinline) (`self.CanPieceMoveToCell` _output_get (`local.CaptureMode`)))
        (set `local.Loop` (not _lastinline))
        (if _result
          (`KismetArrayLibrary.Array_Add` (`local.Output`) (`local.CurrentCell`))))))
  (return (`local.Output`)))

(fn `HasPieceBeenMoved`
  (returns (HasBeenMoved :type Boolean))
  (return (`self.HasBeenMoved`)))

(fn `PotentialMoveList`
  (params (StartCell :type "/Game/3PGame/Blueprints/Board/3PCell Structure"))
  (returns (EndCell :type "Array of /Game/3PGame/Blueprints/Board/3PCell Structure"))
  (return))

(fn `UserConstructionScript`)