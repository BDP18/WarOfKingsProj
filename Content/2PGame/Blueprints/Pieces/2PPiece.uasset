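; Base piece for a two-player chess-style board game, tinted and rotated on BeginPlay for its owning player.
; PotentialMoveList is an empty stub, alongside helpers that gather cells for single-step moves or directional slides.
; Both helpers mirror offsets by player through CellAfterMoved, then CanPieceMoveToCell checks the board for validity, occupancy and capture mode, flagging where slides stop.
; It also tracks has-moved and en passant vulnerability state.
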(event `self.ReceiveBeginPlay`
  (bind _returnvalue (`KismetMaterialLibrary.CreateDynamicMaterialInstance` "/Game/Boardgame_Collection/Materials/Realistic/MI_White.MI_White"))
  (`PrimitiveComponent.SetMaterial` (`self.StaticMesh`) 0 _returnvalue)
  (`MaterialInstanceDynamic.SetVectorParameterValue` _returnvalue "Color" (`/Game/2PGame/Blueprints/2PChessLibrary.PlayerColor` (`self.CurrentPlayerIndex`)))
  (if (== (`self.CurrentPlayerIndex`) 1)
    (`self.K2_SetActorRotation` (struct :`Yaw` -90.0))
    (else
      (`self.K2_SetActorRotation` (struct :`Yaw` 90.0)))))

(event `WhenMoved`
  (set `self.HasBeenMoved` true))

(event `self.StaticMesh.OnBeginCursorOver`
  (params (TouchedComponent :type "PrimitiveComponent Object Reference")))

(fn `CanPieceMoveToCell`
  (params (Cell :type "/Game/2PGame/Blueprints/Board/2PCell Structure") (CaptureMode :type "/Game/2PGame/Blueprints/2PCaptureMode Enum" :default "NewEnumerator0"))
  (returns (Result :type Boolean) (LastInLine :type Boolean))
  (locals (`LastInLine (local)` :type Boolean) (`Add (local)` :type Boolean))
  (`|ExecutionSequence`
    (:`then_0`
      (bind (_tilevalid _tilefree _boardpiece) (`/Game/2PGame/Blueprints/Board/2PBoard.GetCellInfo` (`/Game/2PGame/Blueprints/2PChessLibrary.Board`) (`local.Cell`)))
      (if _tilevalid
        (if _tilefree
          (if (`|EnumEquality` (`local.CaptureMode`) "NewEnumerator2")
            (set `local.LastInLine (local)` true)
            (else
              (set `local.Add (local)` true :!label _label)))
          (else
            (set `local.LastInLine (local)` true)
            (if (and (`|EnumInequality` (`local.CaptureMode`) "NewEnumerator1") (!= (`/Game/2PGame/Blueprints/Pieces/2PPiece.CurrentPlayerIndex` _boardpiece) (`self.CurrentPlayerIndex`)))
              (goto _label))))
        (else
          (set `local.LastInLine (local)` true))))
    (:`then_1`
      (return (`local.Add (local)`) (`local.LastInLine (local)`)))))

(fn `CellAfterMoved`
  (params (Cell :type "/Game/2PGame/Blueprints/Board/2PCell Structure") (Forward :type Integer :default 1) (Right :type Integer))
  (returns (NewCell :type "/Game/2PGame/Blueprints/Board/2PCell Structure"))
  (bind _returnvalue (select `int` (`self.CurrentPlayerIndex`) :`0` 1 :`1` -1))
  (return (make `/Game/2PGame/Blueprints/Board/2PCell` (+ Cell_Col_2_767D76F24B6395F8CD2202A2E588D57E (* (`local.Right`) _returnvalue)) (+ Cell_Row_4_A31AD37F4ABEE7282C2022A30B0EBA3F (* _returnvalue (`local.Forward`))))))

(fn `GetCellsFromMove`
  (params (Cell :type "/Game/2PGame/Blueprints/Board/2PCell Structure") (Forward :type Integer) (Right :type Integer) (CaptureMode :type "/Game/2PGame/Blueprints/2PCaptureMode Enum" :default "NewEnumerator0"))
  (returns (Cells :type "Array of /Game/2PGame/Blueprints/Board/2PCell Structure"))
  (locals (CurrentCell :type "/Game/2PGame/Blueprints/Board/2PCell Structure"))
  (bind _newcell (`self.CellAfterMoved` Cell Forward Right))
  (bind _output_get (set `local.CurrentCell` _newcell))
  (bind _result (`self.CanPieceMoveToCell` _output_get (`local.CaptureMode`)))
  (if _result
    (return (`|MakeArray` (`local.CurrentCell`)))
    (else
      (return))))

(fn `GetCellsFromSlide`
  (params (Cell :type "/Game/2PGame/Blueprints/Board/2PCell Structure") (Direction :type "/Game/2PGame/Blueprints/2PMovement Enum" :default "NewEnumerator0") (MaxDistance :type Integer) (Capture :type "/Game/2PGame/Blueprints/2PCaptureMode Enum" :default "NewEnumerator0"))
  (returns (CellPath :type "Array of /Game/2PGame/Blueprints/Board/2PCell Structure"))
  (locals (CurrentCell :type "/Game/2PGame/Blueprints/Board/2PCell Structure") (Loop :type Boolean :default true) (Output :type "Array of /Game/2PGame/Blueprints/Board/2PCell Structure") (Distance :type Integer))
  (set `local.CurrentCell` Cell)
  (while (and (`local.Loop`) (< (`local.Distance`) (`local.MaxDistance`)))
    (`/Engine/EditorBlueprintResources/StandardMacros.IncrementInt` (`local.Distance`)
      (:`  `
        (bind _newcell (`self.CellAfterMoved` (`local.CurrentCell`) (select `/Game/2PGame/Blueprints/2PMovement` (`local.Direction`) :`NewEnumerator0` 1 :`NewEnumerator4` 1 :`NewEnumerator1` -1 :`NewEnumerator2` -1 :`NewEnumerator5` -1 :`NewEnumerator7` 1) (select `/Game/2PGame/Blueprints/2PMovement` (`local.Direction`) :`NewEnumerator4` 1 :`NewEnumerator3` 1 :`NewEnumerator1` 1 :`NewEnumerator5` -1 :`NewEnumerator6` -1 :`NewEnumerator7` -1)))
        (bind _output_get (set `local.CurrentCell` _newcell))
        (bind (_result _lastinline) (`self.CanPieceMoveToCell` _output_get (`local.Capture`)))
        (set `local.Loop` (not _lastinline))
        (if _result
          (`KismetArrayLibrary.Array_Add` (`local.Output`) (`local.CurrentCell`))))))
  (return (`local.Output`)))

(fn `GetEnPassantVulnerable`
  (returns (EnPassantVulnerable :type Boolean))
  (return (`self.EnPassantVulnerable`)))

(fn `HasPieceBeenMoved`
  (returns (HasBeenMoved :type Boolean))
  (return (`self.HasBeenMoved`)))

(fn `PotentialMoveList`
  (params (StartCell :type "/Game/2PGame/Blueprints/Board/2PCell Structure"))
  (returns (EndCell :type "Array of /Game/2PGame/Blueprints/Board/2PCell Structure"))
  (return))

(fn `SetEnPassantVulnerable`
  (params (Vulnerable :type Boolean))
  (set `self.EnPassantVulnerable` Vulnerable))

(fn `UserConstructionScript`)