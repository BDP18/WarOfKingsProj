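; King piece Blueprint for the two-player board game, defining which cells the king can potentially move to.
; PotentialMoveList calls GetCellsFromMove for the eight one-step Forward/Right offsets around the start cell, appending each result to the returned list.
; An alternative version using GetCellsFromSlide with a max distance of one is left disconnected and never runs.
; The event graph holds only disabled default events.
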(fn `PotentialMoveList`
  (params (StartCell :type "/Game/2PGame/Blueprints/Board/2PCell Structure"))
  (returns (EndCell :type "Array of /Game/2PGame/Blueprints/Board/2PCell Structure"))
  (locals (Output :type "Array of /Game/2PGame/Blueprints/Board/2PCell Structure"))
  (`|ExecutionSequence`
    (:`then_0`
      (`|ExecutionSequence`
        (:`then_0`
          (bind _cells (`self.GetCellsFromMove` (`local.StartCell`) 1))
          (`KismetArrayLibrary.Array_Append` (`local.Output`) _cells))
        (:`then_1`
          (bind _cells_2 (`self.GetCellsFromMove` (`local.StartCell`) 1 1))
          (`KismetArrayLibrary.Array_Append` (`local.Output`) _cells_2))
        (:`then_2`
          (bind _cells_3 (`self.GetCellsFromMove` (`local.StartCell`) 0 1))
          (`KismetArrayLibrary.Array_Append` (`local.Output`) _cells_3))
        (:`then_3`
          (bind _cells_4 (`self.GetCellsFromMove` (`local.StartCell`) -1 1))
          (`KismetArrayLibrary.Array_Append` (`local.Output`) _cells_4))
        (:`then_4`
          (bind _cells_5 (`self.GetCellsFromMove` (`local.StartCell`) -1))
          (`KismetArrayLibrary.Array_Append` (`local.Output`) _cells_5))
        (:`then_5`
          (bind _cells_6 (`self.GetCellsFromMove` (`local.StartCell`) -1 -1))
          (`KismetArrayLibrary.Array_Append` (`local.Output`) _cells_6))
        (:`then_6`
          (bind _cells_7 (`self.GetCellsFromMove` (`local.StartCell`) 0 -1))
          (`KismetArrayLibrary.Array_Append` (`local.Output`) _cells_7))
        (:`then_7`
          (bind _cells_8 (`self.GetCellsFromMove` (`local.StartCell`) 1 -1))
          (`KismetArrayLibrary.Array_Append` (`local.Output`) _cells_8))))
    (:`then_1`
      (return (`local.Output`)))))

(fn `UserConstructionScript`
  (`parent.UserConstructionScript`))