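; Chess board actor for a two-player game that spawns both sides' Alice pieces on the server at BeginPlay and records them in a 64-slot BoardState array.
; Helper functions convert between world positions and cells, check bounds and report tile occupancy.
; IsMoveAvailable checks destinations against each piece's PotentialMoveList.
; MakeMove teleports the piece, destroys any occupant, then calls MovePiece to write BoardState and notify the piece.
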(event `self.ReceiveBeginPlay`
  (`/Engine/EditorBlueprintResources/ActorMacros.Switch Has Authority` ; Must Stay Here. Handles replication between client and server
    (:`Authority`
      (`KismetArrayLibrary.Array_Resize` (`self.BoardState`) 64)
      (for _index (range 2)
        (`self.MakeKings` _index)
        (`self.MakeQueens` _index)
        (`self.MakeBishops` _index)
        (`self.MakeKnights` _index)
        (`self.MakeRooks` _index)
        (`self.MakePawns` _index)))))

(fn `AddPiece`
  (params (Piece :type "/Game/3DGame/AliceChess/Blueprints/Pieces/AlicePiece Object Reference (by ref)") (Cell :type "/Game/2PGame/Blueprints/Board/2PCell Structure"))
  (`KismetArrayLibrary.Array_Set` (`self.BoardState`) (`self.GetIndexFromCell` Cell) Piece))

(fn `CellToGrid`
  (params (Tile :type "/Game/2PGame/Blueprints/Board/2PCell Structure"))
  (returns (ReturnValue :type "Vector Structure"))
  (return (+ (`KismetMathLibrary.MakeVector` (`self.HandleRow` Tile_Row_4_A31AD37F4ABEE7282C2022A30B0EBA3F) (`self.HandleColumn` Tile_Col_2_767D76F24B6395F8CD2202A2E588D57E)) (`self.GridVector`))))

(fn `GetCellInfo`
  (params (Cell :type "/Game/2PGame/Blueprints/Board/2PCell Structure"))
  (returns (TileValid :type Boolean) (TileFree :type Boolean) (BoardPiece :type "/Game/3DGame/AliceChess/Blueprints/Pieces/AlicePiece Object Reference"))
  (bind _piece (`self.PieceAtLocation` (`local.Cell`)))
  (if (`self.IsCellInRange` Cell)
    (return true (not (`KismetSystemLibrary.IsValid` _piece)) _piece)
    (else
      (return false false null))))

(fn `IsCellInRange`
  (params (Cell :type "/Game/2PGame/Blueprints/Board/2PCell Structure"))
  (returns (InRange :type Boolean))
  (return (and (`KismetMathLibrary.InRange_IntInt` Cell_Col_2_767D76F24B6395F8CD2202A2E588D57E 0 7) (`KismetMathLibrary.InRange_IntInt` Cell_Row_4_A31AD37F4ABEE7282C2022A30B0EBA3F 0 7))))

(fn `IsMoveAvailable`
  (params (StartCell :type "/Game/2PGame/Blueprints/Board/2PCell Structure") (DestinationCell :type "/Game/2PGame/Blueprints/Board/2PCell Structure"))
  (returns (Result :type Boolean))
  (locals (SelectedPiece :type "/Game/3DGame/AliceChess/Blueprints/Pieces/AlicePiece Object Reference"))
  (bind _output_get (set `local.SelectedPiece` (`self.PieceAtLocation` StartCell)))
  (`/Engine/EditorBlueprintResources/StandardMacros.IsValid` _output_get
    (:`Is Valid`
      (return (`KismetArrayLibrary.Array_Contains` (`/Game/3DGame/AliceChess/Blueprints/Pieces/AlicePiece.PotentialMoveList` (`local.SelectedPiece`) (`local.StartCell`)) (`local.DestinationCell`))))
    (:`Is Not Valid`
      (return false))))

(fn `MakeBishops`
  (params (PlayerIndex :type Integer))
  (locals (Row :type Integer) (Col :type Integer))
  (set `local.Row` (select `int` (`local.PlayerIndex`) :`0` 0 :`1` 7))
  (`|ExecutionSequence`
    (:`then_0`
      (set `local.Col` (select `int` (`local.PlayerIndex`) :`0` 2 :`1` 5))
      (bind _returnvalue (`|SpawnActorFromClass` "/Game/3DGame/AliceChess/Blueprints/Pieces/AliceBishop.AliceBishop_C" (`KismetMathLibrary.MakeTransform` (`self.CellToGrid` (make `/Game/2PGame/Blueprints/Board/2PCell` (`local.Col`) (`local.Row`)))) "Undefined" "OverrideRootScale" null (`local.PlayerIndex`) null))
      (`self.AddPiece` _returnvalue (make `/Game/2PGame/Blueprints/Board/2PCell` (`local.Col`) (`local.Row`))))
    (:`then_1`
      (set `local.Col` (select `int` (`local.PlayerIndex`) :`0` 5 :`1` 2))
      (bind _returnvalue_2 (`|SpawnActorFromClass` "/Game/3DGame/AliceChess/Blueprints/Pieces/AliceBishop.AliceBishop_C" (`KismetMathLibrary.MakeTransform` (`self.CellToGrid` (make `/Game/2PGame/Blueprints/Board/2PCell` (`local.Col`) (`local.Row`)))) "Undefined" "OverrideRootScale" null (`local.PlayerIndex`) null))
      (`self.AddPiece` _returnvalue_2 (make `/Game/2PGame/Blueprints/Board/2PCell` (`local.Col`) (`local.Row`))))))

(fn `MakeKings`
  (params (PlayerIndex :type Integer))
  (locals (Row :type Integer) (Col :type Integer))
  (set `local.Row` (select `int` (`local.PlayerIndex`) :`0` 0 :`1` 7))
  (set `local.Col` 4)
  (bind _returnvalue (`|SpawnActorFromClass` "/Game/3DGame/AliceChess/Blueprints/Pieces/AliceKing.AliceKing_C" (`KismetMathLibrary.MakeTransform` (`self.CellToGrid` (make `/Game/2PGame/Blueprints/Board/2PCell` (`local.Col`) (`local.Row`)))) "Undefined" "OverrideRootScale" null (`local.PlayerIndex`) null))
  (`self.AddPiece` _returnvalue (make `/Game/2PGame/Blueprints/Board/2PCell` (`local.Col`) (`local.Row`))))

(fn `MakeKnights`
  (params (PlayerIndex :type Integer))
  (locals (Row :type Integer) (Col :type Integer))
  (set `local.Row` (select `int` (`local.PlayerIndex`) :`0` 0 :`1` 7))
  (`|ExecutionSequence`
    (:`then_0`
      (set `local.Col` (select `int` (`local.PlayerIndex`) :`0` 1 :`1` 6))
      (bind _returnvalue (`|SpawnActorFromClass` "/Game/3DGame/AliceChess/Blueprints/Pieces/AliceKnight.AliceKnight_C" (`KismetMathLibrary.MakeTransform` (`self.CellToGrid` (make `/Game/2PGame/Blueprints/Board/2PCell` (`local.Col`) (`local.Row`)))) "Undefined" "OverrideRootScale" null (`local.PlayerIndex`) null))
      (`self.AddPiece` _returnvalue (make `/Game/2PGame/Blueprints/Board/2PCell` (`local.Col`) (`local.Row`))))
    (:`then_1`
      (set `local.Col` (select `int` (`local.PlayerIndex`) :`0` 6 :`1` 1))
      (bind _returnvalue_2 (`|SpawnActorFromClass` "/Game/3DGame/AliceChess/Blueprints/Pieces/AliceKnight.AliceKnight_C" (`KismetMathLibrary.MakeTransform` (`self.CellToGrid` (make `/Game/2PGame/Blueprints/Board/2PCell` (`local.Col`) (`local.Row`)))) "Undefined" "OverrideRootScale" null (`local.PlayerIndex`) null))
      (`self.AddPiece` _returnvalue_2 (make `/Game/2PGame/Blueprints/Board/2PCell` (`local.Col`) (`local.Row`))))))

(fn `MakeMove`
  (params (StartCell :type "/Game/2PGame/Blueprints/Board/2PCell Structure") (DestinationCell :type "/Game/2PGame/Blueprints/Board/2PCell Structure"))
  (locals (SelectedPiece :type "/Game/3DGame/AliceChess/Blueprints/Pieces/AlicePiece Object Reference") (DestinationPiece :type "/Game/3DGame/AliceChess/Blueprints/Pieces/AlicePiece Object Reference"))
  (set `local.SelectedPiece` (`self.PieceAtLocation` StartCell))
  (set `local.DestinationPiece` (`self.PieceAtLocation` DestinationCell))
  (`self.K2_SetActorLocation` (`local.SelectedPiece`) (`self.CellToGrid` (`local.DestinationCell`)) false true)
  (bind _destinationpiece (`local.DestinationPiece`)
    (:`then`
      (`self.K2_DestroyActor` _destinationpiece))
    (:`else`
      _))
  (`self.MovePiece` (`local.StartCell`) (`local.DestinationCell`)))

(fn `MakePawns`
  (params (PlayerIndex :type Integer))
  (locals (Row :type Integer) (Col :type Integer))
  (set `local.Row` (select `int` (`local.PlayerIndex`) :`0` 1 :`1` 6))
  (for _index (range 8)
    (bind _output_get (set `local.Col` _index))
    (bind _returnvalue (`|SpawnActorFromClass` "/Game/3DGame/AliceChess/Blueprints/Pieces/AlicePawn.AlicePawn_C" (`KismetMathLibrary.MakeTransform` (`self.CellToGrid` (make `/Game/2PGame/Blueprints/Board/2PCell` _output_get (`local.Row`)))) "Undefined" "OverrideRootScale" null (`local.PlayerIndex`) null))
    (`self.AddPiece` _returnvalue (make `/Game/2PGame/Blueprints/Board/2PCell` (`local.Col`) (`local.Row`)))))

(fn `MakeQueens`
  (params (PlayerIndex :type Integer))
  (locals (Row :type Integer) (Col :type Integer))
  (set `local.Row` (select `int` (`local.PlayerIndex`) :`0` 0 :`1` 7))
  (set `local.Col` 3)
  (bind _returnvalue (`|SpawnActorFromClass` "/Game/3DGame/AliceChess/Blueprints/Pieces/AliceQueen.AliceQueen_C" (`KismetMathLibrary.MakeTransform` (`self.CellToGrid` (make `/Game/2PGame/Blueprints/Board/2PCell` (`local.Col`) (`local.Row`)))) "Undefined" "OverrideRootScale" null (`local.PlayerIndex`) null))
  (`self.AddPiece` _returnvalue (make `/Game/2PGame/Blueprints/Board/2PCell` (`local.Col`) (`local.Row`))))

(fn `MakeRooks`
  (params (PlayerIndex :type Integer))
  (locals (Row :type Integer) (Col :type Integer))
  (set `local.Row` (select `int` (`local.PlayerIndex`) :`0` 0 :`1` 7))
  (`|ExecutionSequence`
    (:`then_0`
      (set `local.Col` (select `int` (`local.PlayerIndex`) :`0` 0 :`1` 7))
      (bind _returnvalue (`|SpawnActorFromClass` "/Game/3DGame/AliceChess/Blueprints/Pieces/AliceRook.AliceRook_C" (`KismetMathLibrary.MakeTransform` (`self.CellToGrid` (make `/Game/2PGame/Blueprints/Board/2PCell` (`local.Col`) (`local.Row`)))) "Undefined" "OverrideRootScale" null (`local.PlayerIndex`) null))
      (`self.AddPiece` _returnvalue (make `/Game/2PGame/Blueprints/Board/2PCell` (`local.Col`) (`local.Row`))))
    (:`then_1`
      (set `local.Col` (select `int` (`local.PlayerIndex`) :`0` 7 :`1` 0))
      (bind _returnvalue_2 (`|SpawnActorFromClass` "/Game/3DGame/AliceChess/Blueprints/Pieces/AliceRook.AliceRook_C" (`KismetMathLibrary.MakeTransform` (`self.CellToGrid` (make `/Game/2PGame/Blueprints/Board/2PCell` (`local.Col`) (`local.Row`)))) "Undefined" "OverrideRootScale" null (`local.PlayerIndex`) null))
      (`self.AddPiece` _returnvalue_2 (make `/Game/2PGame/Blueprints/Board/2PCell` (`local.Col`) (`local.Row`))))))

(fn `MovePiece`
  (params (StartCell :type "/Game/2PGame/Blueprints/Board/2PCell Structure") (DestinationCell :type "/Game/2PGame/Blueprints/Board/2PCell Structure"))
  (locals (PieceToMove :type "/Game/3DGame/AliceChess/Blueprints/Pieces/AlicePiece Object Reference"))
  (set `local.PieceToMove` (`self.PieceAtLocation` StartCell))
  (`KismetArrayLibrary.Array_Set` (`self.BoardState`) (`self.GetIndexFromCell` (`local.StartCell`)))
  (`KismetArrayLibrary.Array_Set` (`self.BoardState`) (`self.GetIndexFromCell` (`local.DestinationCell`)))
  (`/Game/3DGame/AliceChess/Blueprints/Pieces/AlicePiece.WhenMoved` (`local.PieceToMove`)))

(fn `PieceAtLocation`
  (params (Cell :type "/Game/2PGame/Blueprints/Board/2PCell Structure"))
  (returns (Piece :type "/Game/3DGame/AliceChess/Blueprints/Pieces/AlicePiece Object Reference"))
  (return (`|GetArrayItem` (`self.BoardState`) (`self.GetIndexFromCell` Cell))))

(fn `UserConstructionScript`)

(fn `WorldToGrid`
  (params (WorldLocation :type "Vector Structure"))
  (returns (Cell :type "/Game/2PGame/Blueprints/Board/2PCell Structure") (InBounds :type Boolean))
  (locals (`Row Cell` :type Integer :default 0) (`Column Cell` :type Integer :default 0))
  (bind _lengthofcell (`self.LengthOfCell`))
  (bind (_returnvalue_x _returnvalue_y) (`KismetMathLibrary.BreakVector` (- (`local.WorldLocation`) (`self.GridVector`))))
  (`|ExecutionSequence`
    (:`then_0`
      (set `local.Column Cell` (`KismetMathLibrary.FFloor` (/ _returnvalue_y _lengthofcell)))
      (set `local.Row Cell` (`KismetMathLibrary.FFloor` (/ _returnvalue_x _lengthofcell))))
    (:`then_1`
      (if (`self.IsCellInRange` (make `/Game/2PGame/Blueprints/Board/2PCell` (`local.Column Cell`) (`local.Row Cell`)))
        (return (make `/Game/2PGame/Blueprints/Board/2PCell` (`local.Column Cell`) (`local.Row Cell`)) true)
        (else
          (return (struct) false))))))