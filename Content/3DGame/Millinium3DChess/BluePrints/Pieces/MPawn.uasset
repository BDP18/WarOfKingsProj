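; Pawn piece for a 3D chess game, supplying the list of cells it could move to from a given start cell.
; PotentialMoveList gathers slide results in three forward directions, two cells far until the piece has moved and one cell afterwards.
; It then adds one-cell slides in six angled attack directions under a different capture rule, and returns the combined list.
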(fn `PotentialMoveList`
  (params (StartCell :type "/Game/3DGame/Millinium3DChess/BluePrints/Board/MCell Structure"))
  (returns (EndCell :type "Array of /Game/3DGame/Millinium3DChess/BluePrints/Board/MCell Structure"))
  (locals (Output :type "Array of /Game/3DGame/Millinium3DChess/BluePrints/Board/MCell Structure"))
  (`|ExecutionSequence`
    (:`then_0`
      (`|ExecutionSequence`
        (:`then_0`
          ;[1 1 1] Move forward 2
          (bind _cellpath (`self.GetCellsFromSlide` (`local.StartCell`) "NewEnumerator0" (select `bool` (`self.HasPieceBeenMoved`) :`false` 2 :`true` 1) "NewEnumerator1"))
          (`KismetArrayLibrary.Array_Append` (`local.Output`) _cellpath)
          ;[1 1 1] Move forward 2
          (bind _cellpath_2 (`self.GetCellsFromSlide` (`local.StartCell`) "NewEnumerator8" (select `bool` (`self.HasPieceBeenMoved`) :`false` 2 :`true` 1) "NewEnumerator1"))
          (`KismetArrayLibrary.Array_Append` (`local.Output`) _cellpath_2)
          ;[1 1 1] Move forward 2
          (bind _cellpath_3 (`self.GetCellsFromSlide` (`local.StartCell`) "NewEnumerator16" (select `bool` (`self.HasPieceBeenMoved`) :`false` 2 :`true` 1) "NewEnumerator1"))
          (`KismetArrayLibrary.Array_Append` (`local.Output`) _cellpath_3))
        (:`then_1`
          ;[1 1 1] Attack (angled)
          (bind _cellpath_4 (`self.GetCellsFromSlide` (`local.StartCell`) "NewEnumerator4" 1 "NewEnumerator2"))
          (`KismetArrayLibrary.Array_Append` (`local.Output`) _cellpath_4)
          (bind _cellpath_5 (`self.GetCellsFromSlide` (`local.StartCell`) "NewEnumerator7" 1 "NewEnumerator2"))
          (`KismetArrayLibrary.Array_Append` (`local.Output`) _cellpath_5)
          ;[1 1 1] Attack (angled)
          (bind _cellpath_6 (`self.GetCellsFromSlide` (`local.StartCell`) "NewEnumerator9" 1 "NewEnumerator2"))
          (`KismetArrayLibrary.Array_Append` (`local.Output`) _cellpath_6)
          (bind _cellpath_7 (`self.GetCellsFromSlide` (`local.StartCell`) "NewEnumerator15" 1 "NewEnumerator2"))
          (`KismetArrayLibrary.Array_Append` (`local.Output`) _cellpath_7)
          ;[1 1 1] Attack (angled)
          (bind _cellpath_8 (`self.GetCellsFromSlide` (`local.StartCell`) "NewEnumerator17" 1 "NewEnumerator2"))
          (`KismetArrayLibrary.Array_Append` (`local.Output`) _cellpath_8)
          (bind _cellpath_9 (`self.GetCellsFromSlide` (`local.StartCell`) "NewEnumerator23" 1 "NewEnumerator2"))
          (`KismetArrayLibrary.Array_Append` (`local.Output`) _cellpath_9))))
    (:`then_1`
      (return (`local.Output`)))))

(fn `UserConstructionScript`
  (`parent.UserConstructionScript`))