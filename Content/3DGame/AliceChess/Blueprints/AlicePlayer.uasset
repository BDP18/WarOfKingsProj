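; Player pawn for a 3D Alice Chess game that controls the viewing camera and switches it between boards.
; Axis inputs move the pawn along control-yaw directions and rotate the view, while the mouse wheel zooms by changing spring arm length within limits.
; SwitchBoard shifts the camera back and forth along world Y by a fixed offset, choosing direction from its relative Y.
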(event `Key|MouseScrollDown`
  (params (Key :type "Key Structure"))
  (bind _springarm (`self.SpringArm`))
  (:`Pressed`
    (if (< (`SpringArmComponent.TargetArmLength` (`self.SpringArm`)) (`self.MaxArmLength`))
      (set `SpringArmComponent.TargetArmLength` (+ (`SpringArmComponent.TargetArmLength` _springarm) 50.0) _springarm))))

(event `Key|MouseScrollUp`
  (params (Key :type "Key Structure"))
  (bind _springarm (`self.SpringArm`))
  (:`Pressed`
    (if (> (`SpringArmComponent.TargetArmLength` (`self.SpringArm`)) (`self.MinArmLength`))
      (set `SpringArmComponent.TargetArmLength` (- (`SpringArmComponent.TargetArmLength` _springarm) 50.0) _springarm))))

(event `InputAxis|Forward`
  (params (AxisValue :type "Float (single-precision)"))
  (bind (_returnvalue_roll _returnvalue_pitch _returnvalue_yaw) (`KismetMathLibrary.BreakRotator` (`self.GetControlRotation`)))
  (`self.AddMovementInput` (`KismetMathLibrary.GetForwardVector` (`KismetMathLibrary.MakeRotator` 0.0 0.0 _returnvalue_yaw)) AxisValue))

(event `InputAxis|Right`
  (params (AxisValue :type "Float (single-precision)"))
  (bind (_returnvalue_roll _returnvalue_pitch _returnvalue_yaw) (`KismetMathLibrary.BreakRotator` (`self.GetControlRotation`)))
  (`self.AddMovementInput` (`KismetMathLibrary.GetRightVector` (`KismetMathLibrary.MakeRotator` 0.0 0.0 _returnvalue_yaw)) AxisValue))

(event `InputAxis|Lookup`
  (params (AxisValue :type "Float (single-precision)"))
  (`self.AddControllerPitchInput` AxisValue))

(event `InputAxis|LookRight`
  (params (AxisValue :type "Float (single-precision)"))
  (`self.AddControllerYawInput` AxisValue))

(event `InputAction|SwitchBoard`
  (params (Key :type "Key Structure"))
  (bind _camera (`self.Camera`))
  (bind _returnvalue (`SceneComponent.K2_GetComponentLocation` _camera))
  (bind (_relativelocation_x _relativelocation_y) (`KismetMathLibrary.BreakVector` (`SceneComponent.RelativeLocation` _camera)))
  (:`Pressed`
    (if (< _relativelocation_y 1600.0)
      (`KismetSystemLibrary.PrintString` (`KismetStringLibrary.Conv_VectorToString` _returnvalue))
      (`SceneComponent.K2_SetWorldLocation` (`self.Camera`) (+ _returnvalue (0.0 1600.0 0.0)) false false)
      (else
        (`SceneComponent.K2_SetWorldLocation` (`self.Camera`) (- _returnvalue (0.0 1600.0 0.0)) false false)))))

(fn `SetStartingLocation`
  (set `self.CameraLocation` (`SceneComponent.K2_GetComponentLocation` (`self.Camera`))))

(fn `UserConstructionScript`)