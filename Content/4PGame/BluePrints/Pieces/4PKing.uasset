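; King piece Blueprint for the four-player board game, apparently chess, defining which cells the king can move to.
; PotentialMoveList calls GetCellsFromSlide from the start cell once for each of eight directions, capped at a distance of one, and appends the results into one returned list.
; It contains no other logic: the event graph is unused and the construction script only calls its parent.
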(fn `PotentialMoveList`
  (params (StartCell :type "/Game/4PGame/BluePrints/Board/4PCell Structure"))
  (returns (EndCell :type "Array of /Game/4PGame/BluePrints/Board/4PCell Structure"))
  (locals (Output :type "Array of /Game/4PGame/BluePrints/Board/4PCell Structure"))
  (`|ExecutionSequence`
    (:`then_0`
      (`|ExecutionSequence`
        (:`then_0`
          (bind _cellpath (`self.GetCellsFromSlide` (`local.StartCell`) "NewEnumerator0" 1))
          (`KismetArrayLibrary.Array_Append` (`local.Output`) _cellpath))
        (:`then_1`
          (bind _cellpath_2 (`self.GetCellsFromSlide` (`local.StartCell`) "NewEnumerator4" 1))
          (`KismetArrayLibrary.Array_Append` (`local.Output`) _cellpath_2))
        (:`then_2`
          (bind _cellpath_3 (`self.GetCellsFromSlide` (`local.StartCell`) "NewEnumerator3" 1))
          (`KismetArrayLibrary.Array_Append` (`local.Output`) _cellpath_3))
        (:`then_3`
          (bind _cellpath_4 (`self.GetCellsFromSlide` (`local.StartCell`) "NewEnumerator1" 1))
          (`KismetArrayLibrary.Array_Append` (`local.Output`) _cellpath_4))
        (:`then_4`
          (bind _cellpath_5 (`self.GetCellsFromSlide` (`local.StartCell`) "NewEnumerator2" 1))
          (`KismetArrayLibrary.Array_Append` (`local.Output`) _cellpath_5))
        (:`then_5`
          (bind _cellpath_6 (`self.GetCellsFromSlide` (`local.StartCell`) "NewEnumerator5" 1))
          (`KismetArrayLibrary.Array_Append` (`local.Output`) _cellpath_6))
        (:`then_6`
          (bind _cellpath_7 (`self.GetCellsFromSlide` (`local.StartCell`) "NewEnumerator6" 1))
          (`KismetArrayLibrary.Array_Append` (`local.Output`) _cellpath_7))
        (:`then_7`
          (bind _cellpath_8 (`self.GetCellsFromSlide` (`local.StartCell`) "NewEnumerator7" 1))
          (`KismetArrayLibrary.Array_Append` (`local.Output`) _cellpath_8))))
    (:`then_1`
      (return (`local.Output`)))))

(fn `UserConstructionScript`
  (`parent.UserConstructionScript`))